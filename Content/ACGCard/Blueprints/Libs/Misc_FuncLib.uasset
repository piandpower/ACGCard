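; Miscellaneous Blueprint function library of helpers for the ACGCard card game.
; Traces the cursor to a hit actor and location, and finds a player's CardGameCamera by matching auto-activate index to CardGamePlayerId.
; Maps the CardManagerComponent PlayerId to self and opponent IDs.
; Eases widget transforms toward a goal, snapping and reporting arrival when translation and scale lengths and angle nearly match, comparing magnitudes rather than components.
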(fn `2DInterpToGoalLocation`
  (params (CurrentTransform :type "WidgetTransform Structure") (GoalTransform :type "WidgetTransform Structure") (DeltaTIme :type "Float (double-precision)") (InterpSpeed :type "Float (double-precision)"))
  (returns (Transform :type "WidgetTransform Structure") (Arrived :type Boolean))
  (bind ((`Translation` _translation) (`Scale` _scale) (`Angle` _angle)) (break `WidgetTransform` CurrentTransform))
  (bind ((`Translation` _translation_2) (`Scale` _scale_2) (`Angle` _angle_2)) (break `WidgetTransform` GoalTransform))
  (bind _returnvalue (`KismetMathLibrary.Vector2DInterpTo` _translation _translation_2 DeltaTIme InterpSpeed))
  (bind _returnvalue_2 (`KismetMathLibrary.FInterpTo` _angle _angle_2 DeltaTIme InterpSpeed))
  (bind _returnvalue_3 (`KismetMathLibrary.Vector2DInterpTo` _scale _scale_2 DeltaTIme InterpSpeed))
  (bind _returnvalue_4 (and (`KismetMathLibrary.NearlyEqual_FloatFloat` (`KismetMathLibrary.Abs` (`KismetMathLibrary.VSize2D` _returnvalue)) (`KismetMathLibrary.Abs` (`KismetMathLibrary.VSize2D` _translation_2)) 0.001) (`KismetMathLibrary.NearlyEqual_FloatFloat` (`KismetMathLibrary.Abs` (`KismetMathLibrary.VSize2D` _returnvalue_3)) (`KismetMathLibrary.Abs` (`KismetMathLibrary.VSize2D` _scale_2)) 0.001) (`KismetMathLibrary.NearlyEqual_FloatFloat` (`KismetMathLibrary.Abs` _returnvalue_2) (`KismetMathLibrary.Abs` _angle_2) 0.001)))
  (bind _returnvalue_5 (not _returnvalue_4))
  (return (make `WidgetTransform` :`Translation` (select `bool` _returnvalue_5 :`false` _translation_2 :`true` _returnvalue) :`Scale` (select `bool` _returnvalue_5 :`false` _scale_2 :`true` _returnvalue_3) :`Angle` (select `bool` _returnvalue_5 :`false` _angle_2 :`true` _returnvalue_2)) _returnvalue_4))

(fn `GetCardGamePlayerCamera`
  (params (PlayerController :type "/Game/ACGCard/Blueprints/CardGamePlayerController Object Reference"))
  (returns (ChosenCamera :type "/Game/ACGCard/Blueprints/CardGameCamera Object Reference"))
  (bind _ascard_game_player_state (cast `/Game/ACGCard/Blueprints/CardGamePlayerState` (`Controller.PlayerState` PlayerController))
    (:`then`
      (bind _outactors (`GameplayStatics.GetAllActorsOfClass` null "/Game/ACGCard/Blueprints/CardGameCamera.CardGameCamera_C"))
      (for _array_element _outactors
        (if (== (+ (`CameraActor.GetAutoActivatePlayerIndex` _array_element) 1) (`/Game/ACGCard/Blueprints/CardGamePlayerState.CardGamePlayerId` _ascard_game_player_state))
          (return _array_element))))
    (:`CastFailed`
      _))
  (return null))

(fn `GetPlayerIds`
  (params (Controller :type "Controller Object Reference"))
  (returns (`Self Player` :type Integer) (Oppenent :type Integer))
  (switch `int` (`/Game/ACGCard/Blueprints/Components/CardManagerComponent.PlayerId` (`Actor.GetComponentByClass` Controller "/Game/ACGCard/Blueprints/Components/CardManagerComponent.CardManagerComponent_C"))
    (:`0`
      (return 0 1))
    (:`1`
      (return 1 0))))

(fn `MouseToWorldLocation`
  (params (PlatyerController :type "PlayerController Object Reference"))
  (returns (`Hit Result Hit Actor` :type "Actor Object Reference") (`Hit Result Location` :type "Vector Structure"))
  (bind _hitresult (`PlayerController.GetHitResultUnderCursorByChannel` PlatyerController "TraceTypeQuery1" true))
  (return (`.HitActor` (`GameplayStatics.BreakHitResult` _hitresult)) (`.Location` (`GameplayStatics.BreakHitResult` _hitresult))))