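; Blueprint function library of helpers for cards in the ACGCard card game.
; It sets cards up as replicated actors with server-set data, and applies data row and visuals on the client side.
; It also filters placements down to those not full.
; Attack cost is deducted from the controller's turn points whenever they are non-negative, without comparing them to the cost.
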(fn `ComputeCardAttackCost`
  (params (CardControl :type "/Game/ACGCard/Blueprints/Components/CardControComponent Object Reference") (Cost :type Integer))
  (returns (Success :type Boolean))
  (bind _turnpoint (`/Game/ACGCard/Blueprints/Components/CardControComponent.TurnPoint` CardControl))
  (if (>= _turnpoint 0)
    (set `/Game/ACGCard/Blueprints/Components/CardControComponent.TurnPoint` (- _turnpoint Cost) CardControl)
    (return true)
    (else
      (return false))))

(fn `GetAviablePlacement`
  (params (CardPlacement :type "Array of /Game/ACGCard/Blueprints/GamePlay/CardPlacement Object Reference"))
  (returns (`Return AviablePlacement` :type "Array of /Game/ACGCard/Blueprints/GamePlay/CardPlacement Object Reference") (IsAviable :type Boolean))
  (locals (AviablePlacement :type "Array of /Game/ACGCard/Blueprints/GamePlay/CardPlacement Object Reference"))
  (bind _aviableplacement (`local.AviablePlacement`))
  (for _array_element CardPlacement
    (if (not (`/Game/ACGCard/Blueprints/GamePlay/CardPlacement.bIsFull` _array_element))
      (`KismetArrayLibrary.Array_Add` _aviableplacement _array_element)))
  (return _aviableplacement (> (`KismetArrayLibrary.Array_Length` _aviableplacement) 0)))

(fn `SetClientSideData`
  (params (Card :type "/Game/ACGCard/Blueprints/GamePlay/Card Object Reference") (DataRow :type "DataTableRowHandle Structure"))
  (`/Game/ACGCard/Blueprints/GamePlay/Card.SetCardData` :`self` Card :`DataRow` DataRow :`Type` "NewEnumerator1")
  (`/Game/ACGCard/Blueprints/GamePlay/Card.SetCardVisual` Card))

(fn `SetUpCard`
  (params (Card :type "/Game/ACGCard/Blueprints/GamePlay/Card Object Reference") (Struct :type "/Game/ACGCard/Blueprints/Structs/CardStructs/S_Card Structure"))
  (returns (Card1 :type "/Game/ACGCard/Blueprints/GamePlay/Card Object Reference"))
  (`Actor.SetReplicates` Card true)
  (`/Game/ACGCard/Blueprints/GamePlay/Card.Server_SetCardData` Card Struct)
  (return Card))