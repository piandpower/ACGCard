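; Function library of card ability effects for a card game: draw, stat and turn-point boosts, player healing, board damage, cloning and spawning.
; Each function takes a CardControl and ability index, reading parameters from that card's ability struct.
; Clone and random data-table spawns place cards through PlaceCloneCard at a random index in the owner's placement.
; Template, DamageTargetCard and Clone's random-placement branch are empty; board damage only gathers targets for "Self and Opponent".
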(fn `Clone`
  (params (CardControl :type "/Game/ACGCard/Blueprints/Components/CardControl Object Reference") (AbilityIndex :type Integer) (RandomPlacement :type Boolean))
  (locals (GoalPlacement :type "/Game/ACGCard/Blueprints/GamePlay/CardPlacement Object Reference"))
  (bind _ownercard (`/Game/ACGCard/Blueprints/Components/CardControl.OwnerCard` CardControl))
  (bind _returnvalue (`Actor.GetTransform` _ownercard))
  (if RandomPlacement
    (return)
    (else
      (bind _output_get (set `local.GoalPlacement` (`/Game/ACGCard/Blueprints/GamePlay/Card.PlacementOwner` _ownercard)))
      (`/Game/ACGCard/Blueprints/Libs/Card_MacroLib.ServerPlaceCard` (`/Game/ACGCard/Blueprints/Components/CardControl.CardManagerRef` CardControl) (`KismetMathLibrary.MakeTransform` (`KismetMathLibrary.MakeVector` (.x (.location _returnvalue)) (.y (.location _returnvalue)) (+ (.z (.location _returnvalue)) 600.0)) (.rotation _returnvalue) (.scale _returnvalue)) _output_get (`KismetMathLibrary.RandomIntegerInRange` 0 (`KismetArrayLibrary.Array_Length` (`/Game/ACGCard/Blueprints/GamePlay/CardPlacement.Card_Array` _output_get))) (`/Game/ACGCard/Blueprints/GamePlay/Card.PlacementIndex` _ownercard) :!via `Place Clone Card`))))

(fn `DamageTargetCard`
  (params (CardControl :type "/Game/ACGCard/Blueprints/Components/CardControl Object Reference") (AbilityIndex :type Integer)))

(fn `DamgeBoardCard`
  (params (CardControl :type "/Game/ACGCard/Blueprints/Components/CardControl Object Reference") (AbilityIndex :type Integer))
  (locals (Temp_Array :type "Array of /Game/ACGCard/Blueprints/Components/CardControl Object Reference"))
  (bind _temp_array (`local.Temp_Array`))
  (bind (_type _ability_int _trigger _after_use_state _affecting_player) (break `/Game/ACGCard/Blueprints/Structs/CardStructs/S_CardAbility` (`|GetArrayItem` (`/Game/ACGCard/Blueprints/Components/CardControl.AbilityStructRef` CardControl) AbilityIndex)))
  (bind (_self_player _oppenent) (`/Game/ACGCard/Blueprints/Libs/Misc_FuncLib.FilterPlayer` (`/Game/ACGCard/Blueprints/GamePlay/Card.OwnPlayerId` (`/Game/ACGCard/Blueprints/Components/CardControl.OwnerCard` CardControl))))
  (bind _ascard_game_state (cast `/Game/ACGCard/Blueprints/CardGameState` (`GameplayStatics.GetGameState` null))
    (:`then`
      (switch `/Game/ACGCard/Blueprints/Enums/GamePlayEnums/E_Players` _affecting_player
        (:`NewEnumerator0`
          _)
        (:`NewEnumerator1`
          _)
        (:`NewEnumerator2`
          (bind _playerdataarray (`/Game/ACGCard/Blueprints/CardGameState.PlayerDataArray` _ascard_game_state))
          (`KismetArrayLibrary.Array_Append` _temp_array (`/Game/ACGCard/Blueprints/Actor/PlayerDataActor.ActiveCardControl` (`|GetArrayItem` _playerdataarray _self_player)))
          (`KismetArrayLibrary.Array_Append` _temp_array (`/Game/ACGCard/Blueprints/Actor/PlayerDataActor.ActiveCardControl` (`|GetArrayItem` _playerdataarray _oppenent)))))
      (for _array_element (`local.Temp_Array`)
        (if (not (== CardControl _array_element))
          (`/Game/ACGCard/Blueprints/Components/CardControl.TakeDamage` _array_element CardControl _ability_int))))
    (:`CastFailed`
      _))
  (return))

(fn `DrawCard`
  (params (CardControl :type "/Game/ACGCard/Blueprints/Components/CardControl Object Reference") (AbilityIndex :type Integer))
  (`/Game/ACGCard/Blueprints/Components/CardManager.Sever_DrawCard` (`Actor.GetComponentByClass` (`/Game/ACGCard/Blueprints/Libs/Misc_FuncLib.GetPlayerControlByID` (`/Game/ACGCard/Blueprints/Components/CardControl.PlayerId` CardControl)) "/Game/ACGCard/Blueprints/Components/CardManager.CardManager_C") (`.Ability_int_5_033B511F4749EA23923F7AA8D69B304D` (break `/Game/ACGCard/Blueprints/Structs/CardStructs/S_CardAbility` (`|GetArrayItem` (`/Game/ACGCard/Blueprints/Components/CardControl.AbilityStructRef` CardControl) AbilityIndex))))
  (return))

(fn `IncreaseAttack`
  (params (CardControl :type "/Game/ACGCard/Blueprints/Components/CardControl Object Reference") (AbilityIndex :type Integer))
  (set `/Game/ACGCard/Blueprints/Components/CardControl.Attack` (+ (`/Game/ACGCard/Blueprints/Components/CardControl.Attack` CardControl) (`.Ability_int_5_033B511F4749EA23923F7AA8D69B304D` (break `/Game/ACGCard/Blueprints/Structs/CardStructs/S_CardAbility` (`|GetArrayItem` (`/Game/ACGCard/Blueprints/Components/CardControl.AbilityStructRef` CardControl) AbilityIndex)))) CardControl)
  (return))

(fn `IncreaseHealth`
  (params (CardControl :type "/Game/ACGCard/Blueprints/Components/CardControl Object Reference") (AbilityIndex :type Integer))
  (set `/Game/ACGCard/Blueprints/Components/CardControl.Health` (+ (`/Game/ACGCard/Blueprints/Components/CardControl.Health` CardControl) (`.Ability_int_5_033B511F4749EA23923F7AA8D69B304D` (break `/Game/ACGCard/Blueprints/Structs/CardStructs/S_CardAbility` (`|GetArrayItem` (`/Game/ACGCard/Blueprints/Components/CardControl.AbilityStructRef` CardControl) AbilityIndex)))) CardControl)
  (return))

(fn `IncreasePlayerHealth`
  (params (CardControl :type "/Game/ACGCard/Blueprints/Components/CardControl Object Reference") (AbilityIndex :type Integer))
  (bind _returnvalue (`Actor.GetComponentByClass` (`/Game/ACGCard/Blueprints/Libs/Misc_FuncLib.GetBoardPlayerByID` (`/Game/ACGCard/Blueprints/Components/CardControl.PlayerId` CardControl)) "/Game/ACGCard/Blueprints/Components/CardControl.CardControl_C"))
  (set `/Game/ACGCard/Blueprints/Components/CardControl.Health` (+ (`/Game/ACGCard/Blueprints/Components/CardControl.Health` _returnvalue) (`.Ability_int_5_033B511F4749EA23923F7AA8D69B304D` (break `/Game/ACGCard/Blueprints/Structs/CardStructs/S_CardAbility` (`|GetArrayItem` (`/Game/ACGCard/Blueprints/Components/CardControl.AbilityStructRef` CardControl) AbilityIndex)))) _returnvalue)
  (return))

(fn `InCreaseTurnPoint`
  (params (CardControl :type "/Game/ACGCard/Blueprints/Components/CardControl Object Reference") (AbilityIndex :type Integer))
  (set `/Game/ACGCard/Blueprints/Components/CardControl.TurnPoint` (+ (`/Game/ACGCard/Blueprints/Components/CardControl.TurnPoint` CardControl) (`.Ability_int_5_033B511F4749EA23923F7AA8D69B304D` (break `/Game/ACGCard/Blueprints/Structs/CardStructs/S_CardAbility` (`|GetArrayItem` (`/Game/ACGCard/Blueprints/Components/CardControl.AbilityStructRef` CardControl) AbilityIndex)))) CardControl))

(fn `Spawn Random Card From Deck`
  (params (CardControl :type "/Game/ACGCard/Blueprints/Components/CardControl Object Reference") (AbilityIndex :type Integer))
  (bind _ownercard (`/Game/ACGCard/Blueprints/Components/CardControl.OwnerCard` CardControl))
  (bind _returnvalue (`Actor.GetTransform` _ownercard))
  (bind _placementowner (`/Game/ACGCard/Blueprints/GamePlay/Card.PlacementOwner` _ownercard))
  (bind (_type _ability_int _trigger _after_use_state _affecting_player _datatablerow _particles _soundcue _datatable) (break `/Game/ACGCard/Blueprints/Structs/CardStructs/S_CardAbility` (`|GetArrayItem` (`/Game/ACGCard/Blueprints/Components/CardControl.AbilityStructRef` CardControl) AbilityIndex)))
  (`/Engine/EditorBlueprintResources/StandardMacros.IsValid` _datatable
    (:`Is Valid`
      (bind _outrownames (`DataTableFunctionLibrary.GetDataTableRowNames` _datatable))
      (bind _output (`/Game/ACGCard/Blueprints/Libs/Misc_MacroLib.GetRandItemsFromArray` _outrownames _ability_int)
        (:`then`
          (bind _returnvalue_2 (`|GetDataTableRow` _datatable _output)
            (:`then`
              (`/Game/ACGCard/Blueprints/Libs/Card_MacroLib.ServerPlaceCard` (`/Game/ACGCard/Blueprints/GamePlay/Card.CardManagerRef` _ownercard) (`KismetMathLibrary.MakeTransform` (`KismetMathLibrary.MakeVector` (.x (.location _returnvalue)) (.y (.location _returnvalue)) (+ (.z (.location _returnvalue)) 600.0)) (.rotation _returnvalue) (.scale _returnvalue)) _placementowner (`KismetMathLibrary.RandomIntegerInRange` 0 (`KismetArrayLibrary.Array_Length` (`/Game/ACGCard/Blueprints/GamePlay/CardPlacement.Card_Array` _placementowner))) 0 _returnvalue_2 :!via `Place Clone Card`))
            (:`RowNotFound`
              (return))))
        (:`Completed`
          (return))))
    (:`Is Not Valid`
      (return))))

(fn `Template`
  (params (CardControl :type "/Game/ACGCard/Blueprints/Components/CardControl Object Reference") (AbilityIndex :type Integer)))