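; Miscellaneous function library for the card game, providing helpers for cursor picking and player camera lookup.
; MouseToWorldLocation runs a complex Visibility trace under the controller's cursor and returns the hit actor and location.
; GetCardGamePlayerCamera searches all CardGameCamera actors for the one whose auto-activate player index plus one equals the CardGamePlayerId in the controller's CardGamePlayerState, returning nothing without a match.
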(fn `GetCardGamePlayerCamera`
  (params (PlayerController :type "/Game/ACGCard/Blueprints/CardGamePlayerController Object Reference"))
  (returns (ChosenCamera :type "/Game/ACGCard/Blueprints/CardGameCamera Object Reference"))
  (bind _ascard_game_player_state (cast `/Game/ACGCard/Blueprints/CardGamePlayerState` (`Controller.PlayerState` PlayerController))
    (:`then`
      (bind _outactors (`GameplayStatics.GetAllActorsOfClass` null "/Game/ACGCard/Blueprints/CardGameCamera.CardGameCamera_C"))
      (for _array_element _outactors
        (if (== (+ (`CameraActor.GetAutoActivatePlayerIndex` _array_element) 1) (`/Game/ACGCard/Blueprints/CardGamePlayerState.CardGamePlayerId` _ascard_game_player_state))
          (return _array_element))))
    (:`CastFailed`
      _))
  (return null))

(fn `MouseToWorldLocation`
  (params (PlatyerController :type "PlayerController Object Reference"))
  (returns (`Hit Result Hit Actor` :type "Actor Object Reference") (`Hit Result Location` :type "Vector Structure"))
  (bind _hitresult (`PlayerController.GetHitResultUnderCursorByChannel` PlatyerController "TraceTypeQuery1" true))
  (return (`.HitActor` (`GameplayStatics.BreakHitResult` _hitresult)) (`.Location` (`GameplayStatics.BreakHitResult` _hitresult))))