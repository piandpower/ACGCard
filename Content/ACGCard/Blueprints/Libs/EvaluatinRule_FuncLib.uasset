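; Function library of evaluation rules for a card game, scoring a receiving card by its abilities.
; RuleCalculateAdditionalAbilityPointOffset sums points per ability, scaled by its integer value and chosen by type and trigger.
; Turn start and end triggers add points for stat increases and more heavily for board damage, while stat increases on taking damage subtract.
; RuleCalculateAttackPoints is an empty stub.
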(fn `RuleCalculateAdditionalAbilityPointOffset`
  (params (RecevingCard :type "/Game/ACGCard/Blueprints/GamePlay/Card Object Reference"))
  (returns (Points :type Integer))
  (locals (ReturnPoints :type Integer))
  (set `local.ReturnPoints` 0)
  (for _array_element (`.Abilities_24_C61306344C728A66F65153B169DAE830` (break `/Game/ACGCard/Blueprints/Structs/CardStructs/S_Card` (`/Game/ACGCard/Blueprints/GamePlay/Card.CardStruct` RecevingCard)))
    (bind (_type _ability_int _trigger) (break `/Game/ACGCard/Blueprints/Structs/CardStructs/S_CardAbility` _array_element))
    (switch `/Game/ACGCard/Blueprints/Enums/CardEnums/E_CardAbilityType` _type
      (:`NewEnumerator1`
        (switch `/Game/ACGCard/Blueprints/Enums/CardEnums/E_CardAblityTrigger` _trigger :!label _label
          (:`NewEnumerator2`
            (set `local.ReturnPoints` (+ (`local.ReturnPoints`) (* 1 _ability_int)) :!label _label_2))
          (:`NewEnumerator3`
            (goto _label_2))
          (:`NewEnumerator4`
            (set `local.ReturnPoints` (- (`local.ReturnPoints`) (* 1 _ability_int))))))
      (:`NewEnumerator4`
        (goto _label))
      (:`NewEnumerator2`
        (goto _label))
      (:`NewEnumerator5`
        (switch `/Game/ACGCard/Blueprints/Enums/CardEnums/E_CardAblityTrigger` _trigger
          (:`NewEnumerator2`
            _)
          (:`NewEnumerator3`
            _))
        (set `local.ReturnPoints` (+ (`local.ReturnPoints`) (* 5 _ability_int))))))
  (return (`local.ReturnPoints`)))

(fn `RuleCalculateAttackPoints`)