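; Blueprint function library that resolves card game controllers, human or AI, to their references and player IDs.
; Getters cast a controller to the player controller and its PlayerState, or to the AI controller and its pawn, returning a Valid flag.
; The server-only ID lookup handles both types, returning -1 on failure.
; Another function derives self and opponent IDs, using 1 for both when the GameMode holds at most one controller.
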(fn `GetAIControllerReference`
  (params (Controller :type "Controller Object Reference"))
  (returns (`AsBp Card Game AIController` :type "/Game/ACGCard/Blueprints/AI/Bp_CardGameAIController Object Reference") (`AsBp Card Game AIPawn` :type "/Game/ACGCard/Blueprints/AI/Bp_CardGameAIPawn Object Reference") (Valid :type Boolean))
  (bind _asbp_card_game_aicontroller (cast `/Game/ACGCard/Blueprints/AI/Bp_CardGameAIController` Controller)
    (:`then`
      (bind _asbp_card_game_aipawn (cast `/Game/ACGCard/Blueprints/AI/Bp_CardGameAIPawn` (`Controller.K2_GetPawn` _asbp_card_game_aicontroller))
        (:`then`
          (return _asbp_card_game_aicontroller _asbp_card_game_aipawn true))
        (:`CastFailed`
          _)))
    (:`CastFailed`
      _))
  (return null null false))

(fn `GetControllerID(Server Only)`
  (params (Controller :type "Controller Object Reference"))
  (returns (ID :type Integer))
  (bind _ascard_game_player_controller (cast `/Game/ACGCard/Blueprints/CardGamePlayerController` Controller)
    (:`then`
      (bind _ascard_game_player_state (cast `/Game/ACGCard/Blueprints/CardGamePlayerState` (`Controller.PlayerState` _ascard_game_player_controller))
        (:`then`
          (return (`/Game/ACGCard/Blueprints/CardGamePlayerState.CardGamePlayerId` _ascard_game_player_state)))
        (:`CastFailed`
          _)))
    (:`CastFailed`
      (bind _asbp_card_game_aicontroller (cast `/Game/ACGCard/Blueprints/AI/Bp_CardGameAIController` Controller)
        (:`then`
          (bind _asbp_card_game_aipawn (cast `/Game/ACGCard/Blueprints/AI/Bp_CardGameAIPawn` (`Controller.K2_GetPawn` _asbp_card_game_aicontroller))
            (:`then`
              (return (`/Game/ACGCard/Blueprints/AI/Bp_CardGameAIPawn.PlayerId` _asbp_card_game_aipawn)))
            (:`CastFailed`
              _)))
        (:`CastFailed`
          _))))
  (`KismetSystemLibrary.PrintString` null "Failed to get Controller")
  (return -1))

(fn `GetControllerIDForBOthPlayers`
  (params (Controller :type "Controller Object Reference"))
  (returns (`Self Player` :type Integer) (Oppenent :type Integer))
  (if (> (`KismetArrayLibrary.Array_Length` (`/Game/ACGCard/Blueprints/CardGameMode.GameControllersArray` (cast `/Game/ACGCard/Blueprints/CardGameMode` (`GameplayStatics.GetGameMode` null) :!pure true))) 1)
    (if (== (`self.GetControllerID(Server Only)` Controller) 1)
      (return 1 2)
      (else
        (return 2 1)))
    (else
      (return 1 1))))

(fn `GetPlayerControllerReference`
  (params (Controller :type "Controller Object Reference"))
  (returns (`AsCard Game Player Controller` :type "/Game/ACGCard/Blueprints/CardGamePlayerController Object Reference") (`AsCard Game Player State` :type "/Game/ACGCard/Blueprints/CardGamePlayerState Object Reference") (Valid :type Boolean))
  (bind _ascard_game_player_controller (cast `/Game/ACGCard/Blueprints/CardGamePlayerController` Controller)
    (:`then`
      (bind _ascard_game_player_state (cast `/Game/ACGCard/Blueprints/CardGamePlayerState` (`Controller.PlayerState` _ascard_game_player_controller))
        (:`then`
          (return _ascard_game_player_controller _ascard_game_player_state true))
        (:`CastFailed`
          _)))
    (:`CastFailed`
      _))
  (return null null false))

(fn `NewFunction_0`
  (params (Object :type "Object Object Reference"))
  (cast `/Game/ACGCard/Blueprints/CardGameMode` Object))