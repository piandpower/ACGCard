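; Game instance for the card game that manages multiplayer sessions, main menu and loading screen.
; Hosting creates a session, optionally LAN, and opens TestMap1 as a listen server; joining falls back to the menu on failure.
; A ChangeGameState macro guards screen switches and removes the main menu, while widgets are created once and reused.
; Showing the menu also destroys any session; network and travel errors are only printed.
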(event `self.ReceiveInit`
  ;[1 1 1] Init
)

(event `HostGame`
  ;[1 1 1] Host Game
  (`self.Show Loading Screen`)
  (`CreateSessionCallbackProxy.CreateSession` (`GameplayStatics.GetPlayerController` 0) 3 (`self.EnableLAN`)
    (:`then`
      (`KismetSystemLibrary.PrintString` "Creating Game Session..."))
    (:`OnSuccess`
      (`GameplayStatics.OpenLevel` "TestMap1" true "Listen")
      (`KismetSystemLibrary.PrintString` "Open LevelMap1"))
    (:`OnFailure`
      (`KismetSystemLibrary.PrintString` "Failed to Create Game Session..." false true (struct :`G` 1.0 :`B` 0.007393 :`A` 1.0) 10.0))))

(event `ShowMainMenuEvent`
  (bind _returnvalue (`GameplayStatics.GetPlayerController` 0))
  (bind _mainmenu (`self.MainMenu`))
  ;[1 1 1] Show Main Menu
  (`self.ChangeGameState` "NewEnumerator1"
    (:`IsSameState`
      _)
    (:`NewState`
      _))
  (`/Engine/EditorBlueprintResources/StandardMacros.IsValid` _mainmenu
    (:`Is Valid`
      _)
    (:`Is Not Valid`
      (bind _returnvalue_2 (`|CreateWidget` "/Game/ACGCard/Blueprints/Widgets/Menu/W_MainMenu.W_MainMenu_C" _returnvalue))
      (set `self.MainMenu` _returnvalue_2)))
  (`UserWidget.AddToViewport` _mainmenu 0)
  (`DestroySessionCallbackProxy.DestroySession` _returnvalue))

(event `Show Loading Screen`
  (bind _loadingscreent (`self.LoadingScreent`))
  ;[1 1 1] Show Loading Screen
  (`self.ChangeGameState` "NewEnumerator2"
    (:`NewState`
      (`/Engine/EditorBlueprintResources/StandardMacros.Can Execute Cosmetic Events`
        (:`True`
          (`/Engine/EditorBlueprintResources/StandardMacros.IsValid` _loadingscreent
            (:`Is Valid`
              _)
            (:`Is Not Valid`
              (bind _returnvalue (`|CreateWidget` "/Game/ACGCard/Blueprints/Widgets/Menu/W_LoadingScreen.W_LoadingScreen_C" (`GameplayStatics.GetPlayerController` 0)))
              (set `self.LoadingScreent` _returnvalue)))
          (`UserWidget.AddToViewport` _loadingscreent 0))))))

(event `JoinSession`
  (params (Session :type "BlueprintSessionResult Structure"))
  ;[1 1 1] Join Session
  (`self.Show Loading Screen`)
  (`JoinSessionCallbackProxy.JoinSession` (`GameplayStatics.GetPlayerController` 0) Session
    (:`then`
      (`KismetSystemLibrary.PrintString` "Joining Game Session..." true true (struct :`G` 1.0 :`B` 0.007393 :`A` 1.0) 5.0))
    (:`OnSuccess`
      (`KismetSystemLibrary.PrintString` "Joined Game Session..." true true (struct :`G` 1.0 :`B` 0.007393 :`A` 1.0) 5.0))
    (:`OnFailure`
      (`KismetSystemLibrary.PrintString` "Failed to Join Game Session..." true true (struct :`R` 1.0 :`B` 0.059079 :`A` 1.0) 5.0)
      (`self.ShowMainMenuEvent`))))

(event `self.HandleNetworkError`
  (params (FailureType :type "ENetworkFailure Enum" :default "NetDriverAlreadyExists") (bIsServer :type Boolean))
  ;[1 1 1] Debug
  (`KismetSystemLibrary.PrintString` (`|GetEnumeratorNameAsString` FailureType)))

(event `self.HandleTravelError`
  (params (FailureType :type "ETravelFailure Enum" :default "NoLevel"))
  ;[1 1 1] Debug
  (`KismetSystemLibrary.PrintString` (`|GetEnumeratorNameAsString` FailureType)))

(fn `BeginPlay`
  (`self.ShowMainMenuEvent`))