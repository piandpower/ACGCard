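; Card manager component that relays card additions and hand UI refreshes to client-side listeners in the card game.
; On BeginPlay it caches the CardGameState and the owner's InteractionComponent, then binds handlers to its AddCard and UpdateUI events.
; The handlers route through client events that fire ClientAddCard and ClientUpdateUI calls for listeners.
; The CardsInHand RepNotify fires the same UI update call when the hand replicates.
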(event `self.ReceiveBeginPlay`
  (bind _returnvalue (`Actor.GetComponentByClass` (`self.GetOwner`) "/Game/ACGCard/Blueprints/Components/InteractionComponent.InteractionComponent_C"))
  (`|ExecutionSequence`
    (:`then_0`
      (`|ExecutionSequence`
        (:`then_0`
          (bind _ascard_game_state (cast `/Game/ACGCard/Blueprints/CardGameState` (`GameplayStatics.GetGameState`)))
          (set `self.CardGameStateRef` _ascard_game_state))
        (:`then_1`
          (`/Engine/EditorBlueprintResources/StandardMacros.IsValid` _returnvalue
            (:`Is Valid`
              (set `self.InteractionRef` _returnvalue))))))
    (:`then_1`
      (`self.Bind Event`))))

(event `Bind Event`
  (add `self.AddCard` (delegate `AddCard_Event`))
  (add `self.UpdateUI` (delegate `UpdateUI_Event`)))

(event `Client Add Card`
  (params (Cards :type "Array of DataTableRowHandle Structure (by ref)"))
  ;[1 1 1] Client Event
  (`self.Client_AddCard` Cards))

(event `AddCard_Event` :!signature `self.AddCard`
  (params (Cards :type "Array of DataTableRowHandle Structure (by ref)"))
  (`self.Client Add Card` Cards))

(event `Client Update UI`
  ;[1 1 1] Client Event
  (`self.Client_UpdateUI`))

(event `UpdateUI_Event`
  (`self.Client Update UI`))

(fn `OnRep_CardsInHand`
  (`self.Client_UpdateUI`))