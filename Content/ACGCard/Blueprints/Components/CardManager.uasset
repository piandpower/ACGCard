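; Per-player card manager component that runs a networked card game's hand, turn and combat logic with server authority.
; Turn changes refresh mana and draw cards at random from the GameState's default cards, paced by a gate and retriggerable delay.
; Playing a card checks mana, removes it from hand and spawns it onto a placement.
; Interactions trade damage through CardControl components, with replication and client events relaying changes.
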(event `self.ReceiveBeginPlay`
  (`/Game/ACGCard/Blueprints/Libs/ActorComponent_MacroLib.OwnerAuthority`
    (:`Authority`
      (`|ExecutionSequence`
        (:`then_0`
          (bind _ascard_game_state (cast `/Game/ACGCard/Blueprints/CardGameState` (`GameplayStatics.GetGameState`)))
          (set `self.CardGameStateRef` _ascard_game_state))
        (:`then_1`
          (bind _ascard_game_mode (cast `/Game/ACGCard/Blueprints/CardGameMode` (`GameplayStatics.GetGameMode`)))
          (set `self.CardGameModeRef` _ascard_game_mode))
        (:`then_2`
          (set `self.Owner` (`self.GetOwner`)))))))

(event `Server_PlayCard`
  (params (Row :type "DataTableRowHandle Structure") (Struct :type "/Game/ACGCard/Blueprints/Structs/CardStructs/S_Card Structure") (CardHandIndex :type Integer) (SpawnTransform :type "Transform Structure") (CardPlacement :type "/Game/ACGCard/Blueprints/GamePlay/CardPlacement Object Reference"))
  (bind _playerdata (`self.PlayerData`))
  (`/Game/ACGCard/Blueprints/Libs/ActorComponent_MacroLib.OwnerAuthority`
    (:`Authority`
      (bind _valid (`self.CheckManaCost` (`.Mana_Cost_5_039364194F7BD84FA063B7AC0DE62423` (break `/Game/ACGCard/Blueprints/Structs/CardStructs/S_CardPlacement` (`.Placement_28_AF5522054A4BACE33587D196F19C0F73` (break `/Game/ACGCard/Blueprints/Structs/CardStructs/S_Card` Struct))))))
      (if _valid
        (`self.RemoveCardFromHand` Row CardHandIndex)
        (bind _returnvalue (`|SpawnActorFromClass` "/Game/ACGCard/Blueprints/GamePlay/Card.Card_C" SpawnTransform "Undefined" "OverrideRootScale" (`self.Owner`) CardPlacement (`self.PlayerId`) Struct _playerdata Row null))
        (`/Game/ACGCard/Blueprints/GamePlay/CardPlacement.AddCardPlacement` CardPlacement _returnvalue)
        (`KismetArrayLibrary.Array_Add` (`/Game/ACGCard/Blueprints/Actor/PlayerDataActor.ActiveCard` _playerdata) _returnvalue)
        (else
          (`self.Server_CardMessage` "NewEnumerator1")))
      (`self.Client_DestoryClientCard`))))

(event `Server_RequestChangeTurn`
  (`/Game/ACGCard/Blueprints/Libs/ActorComponent_MacroLib.OwnerAuthority`
    (:`Authority`
      (bind _ascontroller (cast `Controller` (`self.Owner`)))
      (`/Game/ACGCard/Blueprints/CardGameState.Server_RequestChangeTurnState` (`self.CardGameStateRef`) _ascontroller))))

(event `Server_RunCardInteraction`
  (params (TakingCard :type "/Game/ACGCard/Blueprints/GamePlay/Card Object Reference") (RecevingCard :type "/Game/ACGCard/Blueprints/GamePlay/Card Object Reference") (RecevingPlayer :type "/Game/ACGCard/Blueprints/GamePlay/BoardPlayer Object Reference"))
  (`/Game/ACGCard/Blueprints/Libs/ActorComponent_MacroLib.OwnerAuthority`
    (:`Authority`
      (`self.RunCardInteraction` TakingCard RecevingCard RecevingPlayer))))

(event `Server_UpdateReplicatin`
  (params (Replication :type "/Game/ACGCard/Blueprints/Enums/ReplicationEnum/E_CardManagerReplication Enum" :default "NewEnumerator0"))
  (`self.Server_UpdateReplication` Replication))

(event `Sever_OnChangeTurn`
  (params (`Turn Active` :type Boolean))
  (bind _playerdata (`self.PlayerData`))
  (`/Game/ACGCard/Blueprints/Libs/ActorComponent_MacroLib.OwnerAuthority`
    (:`Authority`
      (`|ExecutionSequence`
        (:`then_0`
          (`self.FilterTurnState` `Turn Active`
            (:`Player`
              (set `self.TurnState` "NewEnumerator0")
              (`/Game/ACGCard/Blueprints/Actor/PlayerDataActor.GetManaForTurn` _playerdata)
              (`self.Sever_DrawCard` (`self.CardsToDrawPerTurn`))
              (`/Engine/EditorBlueprintResources/StandardMacros.IncrementInt` (`/Game/ACGCard/Blueprints/Actor/PlayerDataActor.PlayerTurn` _playerdata)))
            (:`Oppenents`
              (set `self.TurnState` "NewEnumerator1"))))
        (:`then_1`
          (`self.Server_UpdateReplicatin` "NewEnumerator2"))))))

(event `SeverEvent_UpdateReplication`
  (params (Replication :type "/Game/ACGCard/Blueprints/Enums/ReplicationEnum/E_CardManagerReplication Enum" :default "NewEnumerator0"))
  (`self.Server_UpdateReplication` Replication))

(event `Sever_MatchBegin`
  (`/Game/ACGCard/Blueprints/Libs/ActorComponent_MacroLib.OwnerAuthority`
    (:`Authority`
      (`self.Sever_DrawCard` 5))))

(event `Sever_DrawCard`
  (params (Number :type Integer))
  (`/Game/ACGCard/Blueprints/Libs/ActorComponent_MacroLib.OwnerAuthority`
    (:`Authority`
      (bind _output_get (set `self.NumberOfCardsToAdd` (+ (`self.NumberOfCardsToAdd`) Number)))
      (`|ExecutionSequence`
        (:`then_0`
          (goto _label :!via `Open`))
        (:`then_1`
          (`/Engine/EditorBlueprintResources/StandardMacros.Gate` true :!label _label
            (:`Exit`
              (if (> _output_get 0)
                (`|ExecutionSequence`
                  (:`then_0`
                    (`/Engine/EditorBlueprintResources/StandardMacros.DecrementInt` _output_get
                      (:`  `
                        (bind _output (`/Game/ACGCard/Blueprints/Libs/Misc_MacroLib.GetRandItemInArray` (`/Game/ACGCard/Blueprints/CardGameState.DefaultCard` (`self.CardGameStateRef`))))
                        (`KismetArrayLibrary.Array_Add` (`self.CardsInHand`) _output)
                        (`self.Server_UpdateReplicatin` "NewEnumerator1")
                        (`self.ClientDrawCardEnd` _output))))
                  (:`then_1`
                    (`KismetSystemLibrary.RetriggerableDelay` 0.2)
                    (goto _label)))
                (else
                  (goto _label :!via `Close`))))))))))

(event `ClientDrawCardEnd`
  (params (Card :type "DataTableRowHandle Structure"))
  (`self.Client_DrawCardEnd` Card))

(event `ClientEvent_UpdateReplication`
  (params (Replication :type "/Game/ACGCard/Blueprints/Enums/ReplicationEnum/E_CardManagerReplication Enum" :default "NewEnumerator0"))
  (`self.Client_UpdateReplication` Replication))

(event `ClientRemoveCardFromHandEnd`
  (params (CardToRemove :type "/Game/ACGCard/Blueprints/Widgets/GamePlay/W_CardWidget Object Reference") (index :type Integer))
  (`self.Client_RemoveCardFromHandEnd` CardToRemove index))

(fn `AddCard`
  (params (Row :type "DataTableRowHandle Structure (by ref)"))
  (bind _cardsinhand (`self.CardsInHand`))
  (`KismetArrayLibrary.Array_Add` _cardsinhand Row)
  (set `/Game/ACGCard/Blueprints/Actor/PlayerDataActor.CardsInHands` (`KismetArrayLibrary.Array_Length` _cardsinhand) (`self.PlayerData`)))

(fn `AddCardToBoard`
  (params (Card :type "/Game/ACGCard/Blueprints/GamePlay/Card Object Reference") (Board :type "/Game/ACGCard/Blueprints/GamePlay/CardPlacement Object Reference"))
  (`/Game/ACGCard/Blueprints/GamePlay/CardPlacement.AddCardPlacement` Board Card))

(fn `CheckManaCost`
  (params (Mana :type Integer))
  (returns (Valid :type Boolean))
  (bind _playerdata (`self.PlayerData`))
  (if (>= (`/Game/ACGCard/Blueprints/Actor/PlayerDataActor.Mana` _playerdata) Mana)
    (`/Game/ACGCard/Blueprints/Actor/PlayerDataActor.DecreaseMana` _playerdata Mana)
    (return true)
    (else
      (return false))))

(fn `CreatePlaceableCard`
  (params (SpawnTransform :type "Transform Structure") (DataRow :type "DataTableRowHandle Structure"))
  (returns (Output_Get :type "/Game/ACGCard/Blueprints/GamePlay/Card Object Reference")))

(fn `DealAttack`
  (params (TakingCardControl :type "/Game/ACGCard/Blueprints/Components/CardControl Object Reference") (RecevingCardControl :type "/Game/ACGCard/Blueprints/Components/CardControl Object Reference"))
  (returns (Success :type Boolean))
  (bind _success (`/Game/ACGCard/Blueprints/Libs/Cards_FuncLib.ComputeCardAttackCost` TakingCardControl 1))
  (if _success
    (`/Game/ACGCard/Blueprints/Components/CardControl.Multi_Attacking` TakingCardControl RecevingCardControl)
    (`/Game/ACGCard/Blueprints/Components/CardControl.TakeDamage` TakingCardControl RecevingCardControl)
    (`/Game/ACGCard/Blueprints/Components/CardControl.TakeDamage` RecevingCardControl TakingCardControl)
    (return true)
    (else
      (return false))))

(fn `OnRep_CardsInHand`
  (`self.ClientEvent_UpdateReplication` "NewEnumerator1"))

(fn `OnRep_TurnState`)

(fn `RemoveCardFromHand`
  (params (Row :type "DataTableRowHandle Structure") (Index :type Integer))
  (returns (Success :type Boolean))
  (bind _cardsinhand (`self.CardsInHand`))
  (`/Game/ACGCard/Blueprints/Libs/ActorComponent_MacroLib.OwnerAuthority`
    (:`Authority`
      (if (`/Game/ACGCard/Blueprints/Libs/Misc_FuncLib.CompareRow` Row (`|GetArrayItem` _cardsinhand Index))
        (`KismetArrayLibrary.Array_Remove` _cardsinhand Index)
        (`self.Server_UpdateReplicatin` "NewEnumerator1")
        (`self.ClientRemoveCardFromHandEnd` null Index)
        (return true)
        (else
          (return false))))))

(fn `RunCardInteraction`
  (params (TakingCard :type "/Game/ACGCard/Blueprints/GamePlay/Card Object Reference") (RecevingCard :type "/Game/ACGCard/Blueprints/GamePlay/Card Object Reference") (RecevingPlayer :type "/Game/ACGCard/Blueprints/GamePlay/BoardPlayer Object Reference"))
  (bind _returnvalue (`Actor.GetComponentByClass` (`self.InteractionTalkingCard`) "/Game/ACGCard/Blueprints/Components/CardControl.CardControl_C"))
  (`/Game/ACGCard/Blueprints/Libs/ActorComponent_MacroLib.OwnerAuthority`
    (:`Authority`
      (`|ExecutionSequence`
        (:`then_0`
          (set `self.InteractionTalkingCard` TakingCard)
          (set `self.InteracitionRecievingCard` RecevingCard)
          (set `self.InteractionRecievingPlayer` RecevingPlayer))
        (:`then_1`
          (`/Engine/EditorBlueprintResources/StandardMacros.IsValid` (`self.InteractionRecievingPlayer`)
            (:`Is Valid`
              (`self.DealAttack` _returnvalue (`Actor.GetComponentByClass` (`self.InteractionRecievingPlayer`) "/Game/ACGCard/Blueprints/Components/CardControl.CardControl_C")))
            (:`Is Not Valid`
              (`self.DealAttack` _returnvalue (`Actor.GetComponentByClass` (`self.InteracitionRecievingCard`) "/Game/ACGCard/Blueprints/Components/CardControl.CardControl_C")))))))))

(fn `ValidateCardInteraction`
  (params (TakingCardControl :type "/Game/ACGCard/Blueprints/Components/CardControl Object Reference") (RecevingCardControl :type "/Game/ACGCard/Blueprints/Components/CardControl Object Reference"))
  (returns (Success :type Boolean))
  (return true))