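; Card actor component that controls a card's stats, abilities, damage and board movement in a networked card game.
; InitCard copies health, attack, owner and abilities from the card struct.
; Triggers such as arriving on board, damage or death run matching abilities on authority, and OnReps relay stat changes through update dispatchers.
; Multicast attack and placement events open a Tick gate that interpolates the owner toward its goal, returning home after attacks.
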(event `InitCard`
  (params (Card :type "/Game/ACGCard/Blueprints/GamePlay/Card Object Reference"))
  (bind (_name _class _type _rarity _visual _attack _health _abilities) (break `/Game/ACGCard/Blueprints/Structs/CardStructs/S_Card` (`/Game/ACGCard/Blueprints/GamePlay/Card.CardStruct` Card)))
  (bind _valid_objet (`/Game/ACGCard/Blueprints/Libs/Misc_MacroLib.ValidGet` Card)
    (:`Is Valid`
      (set `self.OwnerCard` _valid_objet)
      (`|ExecutionSequence`
        (:`then_0`
          (`|ExecutionSequence`
            (:`then_0`
              (set `self.Health` (`.Health_2_DA3A113246AA94D71D1D6782FC7811DF` (break `/Game/ACGCard/Blueprints/Structs/CardStructs/S_CardHealth` _health))))
            (:`then_1`
              (set `self.Attack` (`.Attack_24_125BAE204FCA6459CACE979AB1687861` (break `/Game/ACGCard/Blueprints/Structs/CardStructs/S_CardAttack` _attack))))
            (:`then_2`
              (set `self.PlayerId` (`/Game/ACGCard/Blueprints/GamePlay/Card.OwnPlayerId` Card)))))
        (:`then_1`
          (`|ExecutionSequence`
            (:`then_0`
              (for _array_element _abilities
                (`KismetArrayLibrary.Array_Add` (`self.AbilityStructRef`) _array_element)
                (bind (_type_2 _ability_int _trigger) (break `/Game/ACGCard/Blueprints/Structs/CardStructs/S_CardAbility` _array_element))
                (`KismetArrayLibrary.Array_Add` (`self.AbilityType`) _type_2)
                (`KismetArrayLibrary.Array_Add` (`self.AbilityTrigger`) _trigger)))
            (:`then_1`
              (set `self.CardManagerRef` (`/Game/ACGCard/Blueprints/GamePlay/Card.CardManagerRef` Card)))))))))

(event `self.ReceiveBeginPlay`
  (`/Game/ACGCard/Blueprints/Libs/ActorComponent_MacroLib.OwnerAuthority`
    (:`Authority`
      (`|ExecutionSequence`
        (:`then_0`
          (set `self.Owner` (`self.GetOwner`)))
        (:`then_1`
          (`self.Bind Event`))))))

(event `Bind Event`)

(event `ArriveAtLocation_Event`
  (bind _cardmovementstate (`self.CardMovementState`))
  (bind _returnvalue (> (`self.TurnPoint`) 0))
  (`|ExecutionSequence`
    (:`then_0`
      (switch `/Game/ACGCard/Blueprints/Enums/CardEnums/E_CardMovement` _cardmovementstate
        (:`NewEnumerator1`
          (`self.CloseGate`)
          (`/Engine/EditorBlueprintResources/StandardMacros.DoOnce` false
            (:`Completed`
              (`self.RunActiveAbility` "NewEnumerator1"))))
        (:`NewEnumerator4`
          (set `self.bIsAttacking` false)
          (if (not _returnvalue)
            (set `self.bCardActive` _returnvalue))
          (`self.PlayMovementAnimation` "NewEnumerator1" (`self.HomeDestination`) (`self.HomeRoation`) 50.0 5.0 12.0))))
    (:`then_1`
      (`self.Client_ArriveToLocation` _cardmovementstate))))

(event `self.ReceiveTick`
  (params (DeltaSeconds :type "Float (single-precision)"))
  (bind (_returnvalue _arrived) (`self.InterpSelfToLocation`))
  (bind (_returnvalue_2 _arrived_2) (`self.InterpSelfToRotation`))
  (set `self.DeltaTime` DeltaSeconds)
  (`/Engine/EditorBlueprintResources/StandardMacros.Gate` true :!label _label
    (:`Exit`
      (`Actor.K2_SetActorTransform` (`self.Owner`) (`KismetMathLibrary.MakeTransform` _returnvalue _returnvalue_2) false false)
      (if (and _arrived _arrived_2)
        (`self.ArriveAtLocation_Event`)))))

(event `OpenGate`
  (goto _label :!via `Open`))

(event `CloseGate`
  (goto _label :!via `Close`))

(event `Multi_Attacking`
  (params (GoalComponent :type "/Game/ACGCard/Blueprints/Components/CardControl Object Reference"))
  (`/Game/ACGCard/Blueprints/Libs/ActorComponent_MacroLib.OwnerAuthority`
    (:`Authority`
      (`/Engine/EditorBlueprintResources/StandardMacros.Can Execute Cosmetic Events`
        (:`True`
          _)))
    (:`Remote`
      _))
  (set `self.bIsAttacking` true)
  (`self.PlayMovementAnimation` "NewEnumerator4" (0.0 0.0 0.0) (struct) 50.0 50.0 12.0 (`self.GetOwner` GoalComponent)))

(event `Multi_PlaceOnBoard`
  (params (Location :type "Vector Structure") (Rotation :type "Rotator Structure"))
  (bind _returnrotation (`/Game/ACGCard/Blueprints/Libs/Misc_FuncLib.GetWorldRotationForPlayer` (struct)))
  (set `self.HomeDestination` Location)
  (if (not (`self.bIsPlaced`))
    (set `self.bIsPlaced` true)
    (`Actor.K2_SetActorRotation` (`self.Owner`) _returnrotation false))
  (set `self.HomeRoation` (`KismetMathLibrary.ComposeRotators` Rotation _returnrotation))
  (`self.PlayMovementAnimation` "NewEnumerator1" (`self.HomeDestination`) (`self.HomeRoation`) 50.0 5.0 12.0))

(event `ClientEvent_UpdateReplication`
  (params (Replication :type "/Game/ACGCard/Blueprints/Enums/ReplicationEnum/E_CardControlReplication Enum" :default "NewEnumerator0"))
  (`self.Client_UpdateReplication` Replication))

(event `ServerEvent_UpdateReplication`
  (params (Replication :type "/Game/ACGCard/Blueprints/Enums/ReplicationEnum/E_CardControlReplication Enum" :default "NewEnumerator0"))
  (`/Game/ACGCard/Blueprints/Libs/ActorComponent_MacroLib.OwnerAuthority`
    (:`Authority`
      (`self.Server_UpdateReplication` Replication))))

(event `Server_ActiveAbility`
  (params (AbilityIndex :type Integer))
  (`/Game/ACGCard/Blueprints/Libs/ActorComponent_MacroLib.OwnerAuthority`
    (:`Authority`
      (`self.RunCardAbility` AbilityIndex))))

(event `Server_RunAbility`
  (params (Trigget :type "/Game/ACGCard/Blueprints/Enums/CardEnums/E_CardAblityTrigger Enum" :default "NewEnumerator0"))
  (`/Game/ACGCard/Blueprints/Libs/ActorComponent_MacroLib.OwnerAuthority`
    (:`Authority`
      (`self.RunActiveAbility` Trigget))))

(fn `InterpSelfToLocation`
  (returns (ReturnValue :type "Vector Structure") (Arrived :type Boolean))
  (bind _goaldestination (`self.GoalDestination`))
  (bind _returnvalue (`Actor.K2_GetActorLocation` (`self.Owner`)))
  (bind _returnvalue_2 (`KismetMathLibrary.NearlyEqual_FloatFloat` (`KismetMathLibrary.VSize` (- _returnvalue _goaldestination)) 0.0 (`self.ErrorTolerance`)))
  (return (select `bool` _returnvalue_2 :`false` (`KismetMathLibrary.VInterpTo` _returnvalue _goaldestination (`self.DeltaTime`) (`self.InterpSpeed`)) :`true` _goaldestination) _returnvalue_2))

(fn `InterpSelfToRotation`
  (returns (ReturnValue :type "Rotator Structure") (Arrived :type Boolean))
  (bind _goalrotation (`self.GoalRotation`))
  (bind _returnvalue (`Actor.K2_GetActorRotation` (`self.Owner`)))
  (bind _returnvalue_2 (== _returnvalue _goalrotation :`ErrorTolerance` (/ (`self.ErrorTolerance`) 5.0)))
  (return (select `bool` _returnvalue_2 :`false` (`KismetMathLibrary.RInterpTo` _returnvalue _goalrotation (`self.DeltaTime`) (`self.InterpSpeed`)) :`true` _goalrotation) _returnvalue_2))

(fn `OnRep_Attack`
  (`self.ServerEvent_UpdateReplication` "NewEnumerator1"))

(fn `OnRep_bCardActive`
  (`self.Client_UpdateReplication` "NewEnumerator4"))

(fn `OnRep_bIsDead`)

(fn `OnRep_Health`
  (`self.ServerEvent_UpdateReplication` "NewEnumerator0"))

(fn `OnRep_TurnPoint`
  (`self.Client_UpdateReplication` "NewEnumerator3"))

(fn `PlayMovementAnimation`
  (params (CardMovementState :type "/Game/ACGCard/Blueprints/Enums/CardEnums/E_CardMovement Enum" :default "NewEnumerator0") (GoalDestination :type "Vector Structure") (GoalRotation :type "Rotator Structure") (Zoffset :type "Float (double-precision)") (ErrorTolerance :type "Float (double-precision)") (InterpSpeed :type "Float (double-precision)") (GoalActor :type "Actor Object Reference"))
  (bind (_returnvalue_x _returnvalue_y _returnvalue_z) (`KismetMathLibrary.BreakVector` (`Actor.K2_GetActorLocation` GoalActor)))
  (set `self.CardMovementState` CardMovementState)
  (`/Engine/EditorBlueprintResources/StandardMacros.IsValid` GoalActor ; Is the goal Actor set to be the goal Location?
    (:`Is Valid`
      (set `self.GoalDestination` (`KismetMathLibrary.MakeVector` _returnvalue_x _returnvalue_y (+ _returnvalue_z Zoffset)))
      (set `self.GoalRotation` (`Actor.K2_GetActorRotation` GoalActor)))
    (:`Is Not Valid`
      (set `self.GoalDestination` GoalDestination)
      (set `self.GoalRotation` GoalRotation)))
  (set `self.ErrorTolerance` ErrorTolerance)
  (set `self.InterpSpeed` InterpSpeed)
  (`self.OpenGate`)
  (return))

(fn `RunCardAbility`
  (params (AbilityIndex :type Integer))
  (returns (success :type Boolean))
  (bind _abilityindex_ref (`self.AbilityIndex_Ref`))
  (`/Game/ACGCard/Blueprints/Libs/ActorComponent_MacroLib.OwnerAuthority`
    (:`Authority`
      (set `self.AbilityIndex_Ref` AbilityIndex)
      (switch `/Game/ACGCard/Blueprints/Enums/CardEnums/E_CardAbilityType` (`|GetArrayItem` (`self.AbilityType`) AbilityIndex)
        (:`NewEnumerator0`
          _)
        (:`NewEnumerator9`
          (`/Game/ACGCard/Blueprints/Libs/Ability_Funlib.DrawCard` self _abilityindex_ref))
        (:`NewEnumerator1`
          (`/Game/ACGCard/Blueprints/Libs/Ability_Funlib.IncreaseAttack` self _abilityindex_ref))
        (:`NewEnumerator4`
          (`/Game/ACGCard/Blueprints/Libs/Ability_Funlib.IncreaseHealth` self _abilityindex_ref))
        (:`NewEnumerator2`
          (`/Game/ACGCard/Blueprints/Libs/Ability_Funlib.IncreasePlayerHealth` self _abilityindex_ref))
        (:`NewEnumerator3`
          (`/Game/ACGCard/Blueprints/Libs/Ability_Funlib.InCreaseTurnPoint` self _abilityindex_ref))
        (:`NewEnumerator10`
          (`/Game/ACGCard/Blueprints/Libs/Ability_Funlib.Clone` self _abilityindex_ref))
        (:`NewEnumerator5`
          (`/Game/ACGCard/Blueprints/Libs/Ability_Funlib.DamgeBoardCard` self _abilityindex_ref))
        (:`NewEnumerator8`
          _)
        (:`NewEnumerator6`
          (`/Game/ACGCard/Blueprints/Libs/Ability_Funlib.Spawn Random Card From Deck` self _abilityindex_ref)))
      (return true))
    (:`Remote`
      (return false))))

(fn `TakeDamage`
  (params (Enemy :type "/Game/ACGCard/Blueprints/Components/CardControl Object Reference") (DamageOverride :type Integer))
  (returns (isDead :type Boolean))
  (set `self.Health` (`KismetMathLibrary.Clamp` (- (`self.Health`) (select `bool` (> DamageOverride 0) :`false` (`/Game/ACGCard/Blueprints/Components/CardControl.Attack` Enemy) :`true` DamageOverride)) 0 10000000))
  (`self.RunActiveAbility` "NewEnumerator4")
  (if (not (> (`self.Health`) 0))
    (bind _output_get (set `self.bIsDead` true))
    (`self.RunActiveAbility` "NewEnumerator5")
    (`self.ServerEvent_UpdateReplication` "NewEnumerator2"))
  (return _output_get))