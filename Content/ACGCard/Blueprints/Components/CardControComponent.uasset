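; Card actor component that animates a card moving to its board slot and lunging at attack targets.
; Multicast events set the goal through PlayMovementAnimation, which opens a Tick gate that interpolates the owner's location and rotation until within tolerance.
; Arrival after an attack sends the card back home, arrival at home closes the gate, and both notify through ClientArriveToLocation.
; The IsDead RepNotify calls ServerOnDead.
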(event `Bind Event`)

(event `self.ReceiveBeginPlay`
  (`/Game/ACGCard/Blueprints/Libs/ActorComponent_MacroLib.OwnerAuthority`
    (:`Authority`
      (`|ExecutionSequence`
        (:`then_0`
          (set `self.Owner` (`self.GetOwner`)))
        (:`then_1`
          (`self.Bind Event`))))))

(event `ArriveAtLocation_Event`
  (bind _cardmovementstate (`self.CardMovementState`))
  (`|ExecutionSequence`
    (:`then_0`
      (switch `/Game/ACGCard/Blueprints/Enums/CardEnums/E_CardMovement` _cardmovementstate
        (:`NewEnumerator1`
          (`self.CloseGate`))
        (:`NewEnumerator4`
          (set `self.bIsAttacking` false)
          (`self.PlayMovementAnimation` "NewEnumerator1" (`self.HomeDestination`) (`self.HomeRoation`) 50.0 5.0 12.0))))
    (:`then_1`
      (`self.Client_ArriveToLocation` _cardmovementstate))))

(event `self.ReceiveTick`
  (params (DeltaSeconds :type "Float (single-precision)"))
  (bind (_returnvalue _arrived) (`self.InterpSelfToLocation`))
  (bind (_returnvalue_2 _arrived_2) (`self.InterpSelfToRotation`))
  (set `self.DeltaTime` DeltaSeconds)
  (`/Engine/EditorBlueprintResources/StandardMacros.Gate` true :!label _label
    (:`Exit`
      (`Actor.K2_SetActorTransform` (`self.Owner`) (`KismetMathLibrary.MakeTransform` _returnvalue _returnvalue_2) false false)
      (if (and _arrived _arrived_2)
        (`self.ArriveAtLocation_Event`)))))

(event `OpenGate`
  (goto _label :!via `Open`))

(event `CloseGate`
  (goto _label :!via `Close`))

(event `Multi_Attacking`
  (params (GoalComponent :type "/Game/ACGCard/Blueprints/Components/CardControComponent Object Reference"))
  (`/Game/ACGCard/Blueprints/Libs/ActorComponent_MacroLib.OwnerAuthority`
    (:`Authority`
      (`/Engine/EditorBlueprintResources/StandardMacros.Can Execute Cosmetic Events`
        (:`True`
          _)))
    (:`Remote`
      _))
  (set `self.bIsAttacking` true)
  (`self.PlayMovementAnimation` "NewEnumerator4" (0.0 0.0 0.0) (struct) 50.0 50.0 12.0 (`self.GetOwner` GoalComponent)))

(event `Multi_PlaceOnBoard`
  (params (Location :type "Vector Structure") (Rotation :type "Rotator Structure"))
  (set `self.HomeDestination` Location)
  (if (not (`self.bIsPlaced`))
    (set `self.bIsPlaced` true)
    (`Actor.K2_SetActorRotation` (`self.Owner`) Rotation false))
  (set `self.HomeRoation` (`KismetMathLibrary.ComposeRotators` Rotation (`/Game/ACGCard/Blueprints/Libs/Misc_FuncLib.GetWorldRotationForPlayer` (struct))))
  (`self.PlayMovementAnimation` "NewEnumerator1" (`self.HomeDestination`) (`self.HomeRoation`) 50.0 5.0 12.0))

(fn `InterpSelfToLocation`
  (returns (ReturnValue :type "Vector Structure") (Arrived :type Boolean))
  (bind _goaldestination (`self.GoalDestination`))
  (bind _returnvalue (`Actor.K2_GetActorLocation` (`self.Owner`)))
  (bind _returnvalue_2 (`KismetMathLibrary.NearlyEqual_FloatFloat` (`KismetMathLibrary.VSize` (- _returnvalue _goaldestination)) 0.0 (`self.ErrorTolerance`)))
  (return (select `bool` _returnvalue_2 :`false` (`KismetMathLibrary.VInterpTo` _returnvalue _goaldestination (`self.DeltaTime`) (`self.InterpSpeed`)) :`true` _goaldestination) _returnvalue_2))

(fn `InterpSelfToRotation`
  (returns (ReturnValue :type "Rotator Structure") (Arrived :type Boolean))
  (bind _goalrotation (`self.GoalRotation`))
  (bind _returnvalue (`Actor.K2_GetActorRotation` (`self.Owner`)))
  (bind _returnvalue_2 (== _returnvalue _goalrotation :`ErrorTolerance` (/ (`self.ErrorTolerance`) 5.0)))
  (return (select `bool` _returnvalue_2 :`false` (`KismetMathLibrary.RInterpTo` _returnvalue _goalrotation (`self.DeltaTime`) (`self.InterpSpeed`)) :`true` _goalrotation) _returnvalue_2))

(fn `OnRep_bIsDead`
  (`self.Server_OnDead` (`self.bIsDead`)))

(fn `OnRep_Health`)

(fn `PlayMovementAnimation`
  (params (CardMovementState :type "/Game/ACGCard/Blueprints/Enums/CardEnums/E_CardMovement Enum" :default "NewEnumerator0") (GoalDestination :type "Vector Structure") (GoalRotation :type "Rotator Structure") (Zoffset :type "Float (double-precision)") (ErrorTolerance :type "Float (double-precision)") (InterpSpeed :type "Float (double-precision)") (GoalActor :type "Actor Object Reference"))
  (bind (_returnvalue_x _returnvalue_y _returnvalue_z) (`KismetMathLibrary.BreakVector` (`Actor.K2_GetActorLocation` GoalActor)))
  (set `self.CardMovementState` CardMovementState)
  (`/Engine/EditorBlueprintResources/StandardMacros.IsValid` GoalActor ; Is the goal Actor set to be the goal Location?
    (:`Is Valid`
      (set `self.GoalDestination` (`KismetMathLibrary.MakeVector` _returnvalue_x _returnvalue_y (+ _returnvalue_z Zoffset)))
      (set `self.GoalRotation` (`Actor.K2_GetActorRotation` GoalActor)))
    (:`Is Not Valid`
      (set `self.GoalDestination` GoalDestination)
      (set `self.GoalRotation` GoalRotation)))
  (set `self.ErrorTolerance` ErrorTolerance)
  (set `self.InterpSpeed` InterpSpeed)
  (`self.OpenGate`)
  (return))