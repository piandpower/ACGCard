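; Targeting indicator actor for drag selection in the card game, drawn from the actor's location to a supplied location.
; SetSelectionProperties stretches NarrowCapsule by distance, places ToLocation at the end, and shows Target only for valid targets.
; Both transformed components take their rotation from a look-at toward the mouse's world hit point, not the supplied location.
; On BeginPlay, it destroys the first instance found if more than one exists.
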(event `self.ReceiveBeginPlay`
  (bind _outactors (`GameplayStatics.GetAllActorsOfClass` "TargetDragSelection_C"))
  (if (> (`KismetArrayLibrary.Array_Length` _outactors) 1)
    (`self.K2_DestroyActor` (`|GetArrayItem` _outactors))))

(event `Set Selection Properties`
  (params (Location :type "Vector Structure") (`Valid Target` :type Boolean))
  (bind _returnvalue (`self.K2_GetActorLocation`))
  (bind _returnvalue_2 (`KismetMathLibrary.VSize` (- Location _returnvalue)))
  (bind _returnvalue_3 (`KismetMathLibrary.MakeRotator` (.pitch (`KismetMathLibrary.FindLookAtRotation` _returnvalue (`.Hit Result Location` (`/Game/ACGCard/Blueprints/Libs/Misc_FuncLib.MouseToWorldLocation` (`GameplayStatics.GetPlayerController` 0))))) 0.0 (+ (.yaw (`KismetMathLibrary.FindLookAtRotation` _returnvalue (`.Hit Result Location` (`/Game/ACGCard/Blueprints/Libs/Misc_FuncLib.MouseToWorldLocation` (`GameplayStatics.GetPlayerController` 0))))) 90.0)))
  (if `Valid Target`
    (`SceneComponent.SetVisibility` (`self.Target`) true false)
    (else
      (`SceneComponent.SetVisibility` (`self.Target`) false false)))
  (`SceneComponent.K2_SetWorldTransform` (`self.NarrowCapsule`) (`KismetMathLibrary.MakeTransform` _returnvalue _returnvalue_3 (`KismetMathLibrary.MakeVector` 1.5 (/ _returnvalue_2 195.0) (/ _returnvalue_2 500.0))) false false)
  (`SceneComponent.K2_SetWorldTransform` (`self.ToLocation`) (`KismetMathLibrary.MakeTransform` Location _returnvalue_3 (2.0 2.0 2.0)) false false))

(fn `UserConstructionScript`)