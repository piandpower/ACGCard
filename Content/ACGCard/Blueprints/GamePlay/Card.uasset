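; Replicated card actor for a card game, showing card art, rarity frame, stats, selection and playable highlights, plus a delayed mouse-over preview on desktop and HTML5.
; The server initializes it through the owner's CardManager, then multicasts visual setup, which builds dynamic materials from the card struct.
; CardControl events drive collision, glows and stat text; on death the server removes it from its placement, hides it and destroys it.
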(event `self.ReceiveBeginPlay`
  (`|ExecutionSequence`
    (:`then_0`
      (`|ExecutionSequence`
        (:`then_0`
          (bind _ascard_game_instance (cast `/Game/ACGCard/Blueprints/CardGameInstance` (`GameplayStatics.GetGameInstance`) :!label _label)
            (:`then`
              (bind (_platform _ismobile_) (`/Game/ACGCard/Blueprints/CardGameInstance.GetCurrentPlatform` _ascard_game_instance))
              (set `self.Platform` _platform)
              (set `self.IsMobile` _ismobile_))
            (:`CastFailed`
              (`KismetSystemLibrary.Delay` 0.2)
              (goto _label))))
        (:`then_1`
          (`PrimitiveComponent.SetCollisionEnabled` (`self.CardBase`) "NoCollision"))))
    (:`then_1`
      (`/Engine/EditorBlueprintResources/ActorMacros.Switch Has Authority`
        (:`Authority`
          (`self.SetCardData`)
          (`self.SetReplicates` true)
          (`self.Multi_SetCardVisual`))))))

(event `Multi_SetCardVisual`
  (`self.SetCardVisual`))

(event `Event_Select`
  (params (SelectPlayerID :type Integer))
  (bind _cardbase (`self.CardBase`))
  (`|ExecutionSequence`
    (:`then_0`
      (if (not (`self.isSelected`))
        (set `self.isSelected` true)
        (`self.SetActorScale3D` (1.15 1.15 1.15))
        (if (== SelectPlayerID (`self.OwnPlayerId`))
          (`PrimitiveComponent.SetMaterial` _cardbase 0 "/Game/ACGCard/Assets/Material/UI/CardGreenGlow_Mat.CardGreenGlow_Mat")
          (else
            (`PrimitiveComponent.SetMaterial` _cardbase 0 "/Game/ACGCard/Assets/Material/UI/CardRedGlow_Mat.CardRedGlow_Mat")))))
    (:`then_1`
      (`self.RemoveMouseOverPreview`))))

(event `Event_UnSelect`
  (`|ExecutionSequence`
    (:`then_0`
      (if (and (not (`/Game/ACGCard/Blueprints/Components/CardControl.bCardActive` (`self.CardControl`))) (`self.isSelected`))
        (`PrimitiveComponent.SetMaterial` (`self.CardBase`) 0 (`self.OuterMaterial`))))
    (:`then_1`
      (set `self.isSelected` false)
      (`self.SetActorScale3D` (1.0 1.0 1.0)))))

(event `self.CardControl.Client_ArriveToLocation`
  (params (MovementState :type "/Game/ACGCard/Blueprints/Enums/CardEnums/E_CardMovement Enum" :default "NewEnumerator0"))
  (switch `/Game/ACGCard/Blueprints/Enums/CardEnums/E_CardMovement` MovementState
    (:`NewEnumerator0`
      _)
    (:`NewEnumerator1`
      _))
  (`PrimitiveComponent.SetCollisionEnabled` (`self.CardBase`) "QueryOnly"))

(event `self.CardControl.Server_UpdateReplication`
  (params (Replication :type "/Game/ACGCard/Blueprints/Enums/ReplicationEnum/E_CardControlReplication Enum" :default "NewEnumerator0"))
  (`/Engine/EditorBlueprintResources/ActorMacros.Switch Has Authority`
    (:`Authority`
      (switch `/Game/ACGCard/Blueprints/Enums/ReplicationEnum/E_CardControlReplication` Replication
        (:`NewEnumerator0`
          (`self.Multi_UpdateVisualState` :!label _label_2))
        (:`NewEnumerator1`
          (goto _label_2))
        (:`NewEnumerator2`
          (if (`/Game/ACGCard/Blueprints/Components/CardControl.bIsDead` (`self.CardControl`))
            (`KismetSystemLibrary.Delay` 1.5)
            (`self.MoveToGraveyard`)
            (`self.SetActorHiddenInGame` true)
            (`KismetSystemLibrary.Delay` 10.0)
            (`self.K2_DestroyActor`)))))))

(event `SetHighlight`
  (params (Condition :type Boolean))
  (bind _cardbase (`self.CardBase`))
  (`/Engine/EditorBlueprintResources/StandardMacros.Can Execute Cosmetic Events`
    (:`True`
      (if Condition
        (`PrimitiveComponent.SetMaterial` _cardbase 0 "/Game/ACGCard/Assets/Material/UI/CardGreenGlow_Mat.CardGreenGlow_Mat")
        (else
          (`PrimitiveComponent.SetMaterial` _cardbase 0 null))))))

(event `self.CardControl.Client_UpdateReplication`
  (params (Replication :type "/Game/ACGCard/Blueprints/Enums/ReplicationEnum/E_CardControlReplication Enum" :default "NewEnumerator0"))
  (bind _cardcontrol (`self.CardControl`))
  (switch `/Game/ACGCard/Blueprints/Enums/ReplicationEnum/E_CardControlReplication` Replication
    (:`NewEnumerator3`
      _)
    (:`NewEnumerator4`
      _))
  (`self.SetHighlight` (and (`/Game/ACGCard/Blueprints/Components/CardControl.bCardActive` _cardcontrol) (> (`/Game/ACGCard/Blueprints/Components/CardControl.TurnPoint` _cardcontrol) 0) (== (`self.OwnPlayerId`) (`/Game/ACGCard/Blueprints/Libs/Misc_FuncLib.GetPlayerIds` (`GameplayStatics.GetPlayerController` 0))))))

(event `self.CardControl.Client_OnSelect`
  (params (IsSelect :type Boolean) (Id :type Integer))
  (if IsSelect
    (`self.Event_Select` Id)
    (else
      (`self.Event_UnSelect`))))

(event `self.ReceiveActorBeginCursorOver`
  (switch `/Game/ACGCard/Blueprints/Enums/SystemEnums/E_Platforms` (`self.Platform`)
    (:`NewEnumerator0`
      _)
    (:`NewEnumerator3`
      _)
    (:`NewEnumerator4`
      _)
    (:`NewEnumerator5`
      _))
  (if (`/Game/ACGCard/Blueprints/Components/CardControl.bIsPlaced` (`self.CardControl`))
    (set `self.PreviewEnabled` true)
    (`KismetSystemLibrary.Delay` 0.5) ; Short Delay before enabling the preview IF the the card is still moused over. (Stops the preview popping up every card it mouses over)
    (if (and (not (`self.isSelected`)) (not (`self.bInGraveyard`)))
      (if (`self.PreviewEnabled`)
        (`/Engine/EditorBlueprintResources/StandardMacros.IsValid` (`self.ViewCardPreview`)
          (:`Is Valid`
            _)
          (:`Is Not Valid`
            (bind _returnvalue (`|CreateWidget` "/Game/ACGCard/Blueprints/Widgets/GamePlay/W_CardPreview.W_CardPreview_C" (`GameplayStatics.GetPlayerController` 0) self))
            (bind _output_get (set `self.ViewCardPreview` _returnvalue))))
        (`/Game/ACGCard/Blueprints/Widgets/GamePlay/W_CardPreview.InitialCardPreview` _output_get (`self.CardStruct`) 1.0)
        (`UserWidget.AddToViewport` _output_get 0)
        (else
          (`self.RemoveMouseOverPreview` :!label _label))))))

(event `self.ReceiveActorEndCursorOver`
  (switch `/Game/ACGCard/Blueprints/Enums/SystemEnums/E_Platforms` (`self.Platform`)
    (:`NewEnumerator0`
      _)
    (:`NewEnumerator3`
      _)
    (:`NewEnumerator4`
      _)
    (:`NewEnumerator5`
      _))
  (if (`/Game/ACGCard/Blueprints/Components/CardControl.bIsPlaced` (`self.CardControl`))
    (goto _label)))

(event `Multi_MoveToGraveyard`
  (`/Engine/EditorBlueprintResources/StandardMacros.Can Execute Cosmetic Events`
    (:`True`
      (`self.RemoveMouseOverPreview`))))

(event `Multi_UpdateVisualState`
  (bind _cardcontrol (`self.CardControl`))
  (`/Game/ACGCard/Blueprints/Libs/Misc_MacroLib.ValidGet` self
    (:`Is Valid`
      (`TextRenderComponent.K2_SetText` (`self.Attack_Text`) (`KismetTextLibrary.Conv_IntToText` (`/Game/ACGCard/Blueprints/Components/CardControl.Attack` _cardcontrol)))
      (`TextRenderComponent.K2_SetText` (`self.Health_Text`) (`KismetTextLibrary.Conv_IntToText` (`/Game/ACGCard/Blueprints/Components/CardControl.Health` _cardcontrol)))
      (`TextRenderComponent.K2_SetText` (`self.ManaCost_Text`) (`KismetTextLibrary.Conv_IntToText` (`/Game/ACGCard/Blueprints/Components/CardControl.Mana` _cardcontrol))))))

(fn `MoveToGraveyard`
  (`/Engine/EditorBlueprintResources/ActorMacros.Switch Has Authority`
    (:`Authority`
      (`|ExecutionSequence`
        (:`then_1`
          (`/Game/ACGCard/Blueprints/GamePlay/CardPlacement.RemoveCardPlacement` (`self.PlacementOwner`) self)
          (`self.Multi_MoveToGraveyard`))))))

(fn `RemoveMouseOverPreview`
  (bind _viewcardpreview (`self.ViewCardPreview`))
  (if (`self.PreviewEnabled`)
    (set `self.PreviewEnabled` false)
    (`/Engine/EditorBlueprintResources/StandardMacros.IsValid` _viewcardpreview
      (:`Is Valid`
        (`Widget.RemoveFromParent` _viewcardpreview))
      (:`Is Not Valid`
        _)))
  (return))

(fn `SetCardData`
  (bind _output_get (set `self.CardManagerRef` (`self.GetComponentByClass` (`self.GetOwner`) "/Game/ACGCard/Blueprints/Components/CardManager.CardManager_C")))
  (set `self.PlayerDataRef` (`/Game/ACGCard/Blueprints/Components/CardManager.PlayerData` _output_get))
  (`/Game/ACGCard/Blueprints/Components/CardControl.InitCard` (`self.CardControl`) self)
  (`self.SetCardVisual`)
  (return))

(fn `SetCardVisual`
  (bind (_name _class _type _rarity _visual) (break `/Game/ACGCard/Blueprints/Structs/CardStructs/S_Card` (`self.CardStruct`)))
  (bind (_frame_texture _image_texture _back_texture _frame_material _image_material _back_material) (break `/Game/ACGCard/Blueprints/Structs/CardStructs/S_CardVisual` _visual))
  (bind _returnvalue (`KismetSystemLibrary.IsValid` _frame_material))
  (bind _returnvalue_2 (`KismetSystemLibrary.IsValid` _image_material))
  (bind _returnvalue_3 (`KismetSystemLibrary.IsValid` _back_material))
  (`/Engine/EditorBlueprintResources/StandardMacros.Can Execute Cosmetic Events`
    (:`True`
      (`|ExecutionSequence`
        (:`then_0`
          (bind _returnvalue_4 (`PrimitiveComponent.CreateDynamicMaterialInstance` (`self.CardBase`) 3 (select `bool` _returnvalue :`false` "/Game/ACGCard/Assets/Material/Card/CardFrame_Mat_Parent.CardFrame_Mat_Parent" :`true` _frame_material :!type "MaterialInterface Object Reference"))) ; Create dynamic Card Frame Material
          (if _returnvalue
            (set `self.CardFrameMaterial` _returnvalue_4)
            (else
              (`MaterialInstanceDynamic.SetTextureParameterValue` _returnvalue_4 "FrameImage" (select `/Game/ACGCard/Blueprints/Enums/CardEnums/E_CardRarity` _rarity :`NewEnumerator0` "/Game/ACGCard/Assets/Texture/CardDesign/CardDesign2.CardDesign2" :`NewEnumerator1` "/Game/ACGCard/Assets/Texture/CardDesign/CardDesign_Green.CardDesign_Green" :`NewEnumerator2` "/Game/ACGCard/Assets/Texture/GamePlay/CardDesign.CardDesign" :`NewEnumerator3` "/Game/ACGCard/Assets/Texture/CardDesign/CardDesign_Purple.CardDesign_Purple" :`NewEnumerator4` "/Game/ACGCard/Assets/Texture/CardDesign/CardDesign_Yellow.CardDesign_Yellow" :!type "Texture Object Reference"))))
          (`PrimitiveComponent.SetMaterial` (`self.CardBase`) 3 _returnvalue_4) ; Set Card Frame Material
        )
        (:`then_1`
          (bind _returnvalue_5 (`PrimitiveComponent.CreateDynamicMaterialInstance` (`self.CardBase`) 1 (select `bool` _returnvalue_2 :`false` "/Game/ACGCard/Assets/Material/Card/Card_Mat_Parent.Card_Mat_Parent" :`true` _image_material :!type "MaterialInterface Object Reference"))) ; Create dynamic Card Image Material
          (if _returnvalue_2
            (set `self.CardImageMaterial` _returnvalue_5)
            (else
              (`MaterialInstanceDynamic.SetTextureParameterValue` _returnvalue_5 "CardImage" _image_texture)))
          (`PrimitiveComponent.SetMaterial` (`self.CardBase`) 1 _returnvalue_5) ; Set Card Image Material
        )
        (:`then_2`
          (bind _returnvalue_6 (`PrimitiveComponent.CreateDynamicMaterialInstance` (`self.CardBase`) 2 (select `bool` _returnvalue_3 :`false` "/Game/ACGCard/Assets/Material/Card/CardFrame_Mat_Parent.CardFrame_Mat_Parent" :`true` _back_material :!type "MaterialInterface Object Reference"))) ; Create dynamic Card Back Material
          (if _returnvalue_3
            (set `self.CardBackMaterial` _returnvalue_6)
            (else
              (`MaterialInstanceDynamic.SetTextureParameterValue` _returnvalue_6 "FrameImage" "/Game/ACGCard/Assets/Texture/GamePlay/CardBacking.CardBacking")))
          (`PrimitiveComponent.SetMaterial` (`self.CardBase`) 2 _returnvalue_6) ; Set Card Back Material
        )
        (:`then_3`
          (return))))
    (:`False`
      (return))))

(fn `UserConstructionScript`)