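; Board representation of a player in the card game, showing that player's health as text.
; On BeginPlay the server polls with short delays until the CardGameState and PlayerData for its PlayerIndex are valid, then seeds health into CardConrol.
; CardConrol replication events copy health into PlayerHealth, whose OnRep refreshes the text where cosmetic events can execute.
; Death only prints a debug message.
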(event `self.ReceiveBeginPlay`
  (bind _playerindex (`self.PlayerIndex`))
  (bind _playerdataarray (`/Game/ACGCard/Blueprints/CardGameState.PlayerDataArray` (`self.GameState`)))
  (`/Engine/EditorBlueprintResources/ActorMacros.Switch Has Authority`
    (:`Authority`
      (bind _ascard_game_state (cast `/Game/ACGCard/Blueprints/CardGameState` (`GameplayStatics.GetGameState`) :!label _label)
        (:`then`
          (set `self.GameState` _ascard_game_state)
          (if (> (`KismetArrayLibrary.Array_Length` _playerdataarray) _playerindex) :!label _label_2
            (bind _valid_objet (`/Game/ACGCard/Blueprints/Libs/Misc_MacroLib.ValidGet` (`|GetArrayItem` _playerdataarray _playerindex))
              (:`Is Valid`
                (set `self.PlayerData` _valid_objet)
                (set `/Game/ACGCard/Blueprints/Components/CardControl.Health` (`/Game/ACGCard/Blueprints/Actor/PlayerDataActor.Health` (`self.PlayerData`)) (`self.CardConrol`)))
              (:`Is Not Valid`
                (`KismetSystemLibrary.Delay` 0.2 :!label _label_3)
                (goto _label_2)))
            (else
              (goto _label_3))))
        (:`CastFailed`
          (`KismetSystemLibrary.Delay` 0.2)
          (goto _label))))))

(event `UpdatePlayerStats`
  ;[1 1 1] Comment
  (`/Engine/EditorBlueprintResources/StandardMacros.Can Execute Cosmetic Events`
    (:`True`
      (`TextRenderComponent.K2_SetText` (`self.Health_Text`) (`KismetSystemLibrary.MakeLiteralText` (`KismetTextLibrary.Conv_IntToText` (`self.Player_Health`)))))))

(event `self.CardConrol.Server_UpdateReplication`
  (params (Replication :type "/Game/ACGCard/Blueprints/Enums/ReplicationEnum/E_CardControlReplication Enum" :default "NewEnumerator0"))
  (bind _cardconrol (`self.CardConrol`))
  (switch `/Game/ACGCard/Blueprints/Enums/ReplicationEnum/E_CardControlReplication` Replication
    (:`NewEnumerator0`
      (set `self.Player_Health` (`/Game/ACGCard/Blueprints/Components/CardControl.Health` _cardconrol)))
    (:`NewEnumerator2`
      (if (`/Game/ACGCard/Blueprints/Components/CardControl.bIsDead` _cardconrol)
        (`KismetSystemLibrary.PrintString` "Player Dead")))))

(fn `OnRep_Player_Health`
  (`self.UpdatePlayerStats`))

(fn `UserConstructionScript`)