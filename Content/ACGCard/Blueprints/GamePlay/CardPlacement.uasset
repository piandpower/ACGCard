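; CardPlacement is a board slot actor for a card game that holds cards and lays them out in a row.
; The construction script builds end, middle or single tiles from the placement width and sizes the collision to match.
; AddCardPlacement stores a card, updates IsFull and repositions every card through its CardControComponent.
; Layout uses fixed or dynamically compressed spacing, optionally centred or inverted, with a slight roll when cards overlap.
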(event `AddCardPlacement`
  (params (Card :type "/Game/ACGCard/Blueprints/GamePlay/Card Object Reference"))
  (bind _card_array (`self.Card_Array`))
  (bind _card_array_2 (`self.Card_Array`))
  (`KismetArrayLibrary.Array_Add` _card_array Card)
  (set `self.bIsFull` (>= (`KismetArrayLibrary.Array_Length` _card_array) (`self.MaxCardsInPlacement`)))
  (for (_array_element _array_index) _card_array_2
    (bind (_returnvector _returnrotation) (`self.GetCardInPlacementLocation` _array_index (`self.MaxCardsInPlacement`) (`KismetArrayLibrary.Array_Length` _card_array_2)))
    (`/Game/ACGCard/Blueprints/Components/CardControComponent.Multi_PlaceOnBoard` (`self.GetComponentByClass` _array_element "/Game/ACGCard/Blueprints/Components/CardControComponent.CardControComponent_C") _returnvector _returnrotation)))

(fn `CalculateDynamicSpacingLocation`
  (params (index :type Integer) (`Max Cards In Placement` :type Integer) (`Cards In Placement` :type Integer) (`Center Out` :type Boolean))
  (returns (ReturnValue :type "Float (double-precision)") (Overlap :type Boolean))
  (bind _returnvalue (`KismetMathLibrary.Conv_IntToDouble` `Cards In Placement`))
  (bind _returnvalue_2 (`KismetMathLibrary.Conv_IntToDouble` index))
  (bind _cardspacing (`self.CardSpacing`))
  (bind _returnvalue_3 (- _returnvalue 1.0))
  (bind _returnvalue_4 (* _cardspacing (`KismetMathLibrary.Conv_IntToDouble` `Max Cards In Placement`)))
  (bind _returnvalue_5 (* (select `bool` `Center Out` :`false` _returnvalue_2 :`true` (- _returnvalue_2 (- (/ (select `bool` `Center Out` :`false` (`KismetMathLibrary.Conv_IntToDouble` `Max Cards In Placement`) :`true` (`KismetMathLibrary.Conv_IntToDouble` `Cards In Placement`)) 2.0) 0.5))) (`KismetMathLibrary.FClamp` (/ (- _returnvalue_4 _cardspacing) (select `bool` (>= _returnvalue_3 1.0) :`false` 1.0 :`true` _returnvalue_3)) 0.0 (`self.CardWidth`))))
  (return (select `bool` `Center Out` :`false` (- _returnvalue_5 (- (/ _returnvalue_4 2.0) (/ _cardspacing 2.0))) :`true` _returnvalue_5) (< (- _returnvalue 2.0) (- (`KismetMathLibrary.Conv_IntToDouble` (`KismetMathLibrary.FFloor` (/ _returnvalue_4 (`self.CardWidth`)))) 1.0))))

(fn `CalculateSpacingLocation`
  (params (index :type Integer) (`Max Cards in placement` :type Integer) (`Cards in Placement` :type Integer) (spacing :type "Float (double-precision)"))
  (returns (ReturnValue :type "Float (double-precision)"))
  (return (* (- (`KismetMathLibrary.Conv_IntToDouble` index) (- (/ (select `bool` (`self.bCenterOut`) :`false` (`KismetMathLibrary.Conv_IntToDouble` `Max Cards in placement`) :`true` (`KismetMathLibrary.Conv_IntToDouble` `Cards in Placement`)) 2.0) 0.5)) spacing)))

(fn `CreateVisualBoardTiles`
  (bind _returnvalue (`KismetMathLibrary.FFloor` (`self.PlacementWidth`)))
  (bind _returnvalue_2 (- _returnvalue 1))
  (if (`self.bScaleMulticardPlacement`)
    (for _index (range (+ _returnvalue_2 1))
      (bind _returnvalue_3 (`AddComponent|NODE_AddChildActorComponent-0` :`RelativeTransform` (`KismetMathLibrary.Conv_VectorToTransform` (`KismetMathLibrary.MakeVector` 0.0 (* (- (`KismetMathLibrary.Conv_IntToDouble` _index) (/ (`KismetMathLibrary.Conv_IntToDouble` _returnvalue_2) 2.0)) (`self.CardWidth`))))))
      (`ChildActorComponent.SetChildActorClass` _returnvalue_3 (select `bool` (== _returnvalue 1) :`false` (select `bool` (== _index 0) :`false` (select `bool` (== _index _returnvalue_2) :`false` (`self.MiddleTile`) :`true` (`self.RightEndTile`)) :`true` (`self.LeftEndTile`)) :`true` (`self.SingleTIle`))))))

(fn `GetCardInPlacementLocation`
  (params (index :type Integer) (`Max Cards in placement` :type Integer) (`Cards in Placement` :type Integer))
  (returns (ReturnVector :type "Vector Structure") (ReturnRotation :type "Rotator Structure"))
  (bind _bmultiplacement (`self.bMultiPlacement`))
  (bind (_returnvalue _overlap) (`self.CalculateDynamicSpacingLocation` index `Max Cards in placement` `Cards in Placement` (`self.bCenterOut`)))
  (bind (_returnvalue_roll _returnvalue_pitch _returnvalue_yaw) (`KismetMathLibrary.BreakRotator` (`self.K2_GetActorRotation` self)))
  (bind _returnvalue_2 (`self.K2_GetActorLocation` self))
  (bind _returnvalue_3 (* _returnvalue_2 (1.0 1.0 1.0)))
  (bind _returnvalue_4 (select `bool` (`self.bScaleMulticardPlacement`) :`true` (select `bool` (`self.bDynamicSpacing`) :`false` (`self.CalculateSpacingLocation` index `Max Cards in placement` `Cards in Placement` (`self.CardSpacing`)) :`true` _returnvalue)))
  (bind _returnvalue_5 (select `bool` (and (select `bool` (`self.bDynamicSpacing`) :`false` (<= (`self.CardWidth`) (`self.CardSpacing`)) :`true` _overlap) (>= `Cards in Placement` 1)) :`false` 2.0 :!type "Float (single-precision)"))
  (return (select `bool` (`self.bMultiPlacement`) :`false` (+ _returnvalue_3 (0.0 0.0 10.0)) :`true` (+ (`KismetMathLibrary.GreaterGreater_VectorRotator` (`KismetMathLibrary.MakeVector` (select `bool` _bmultiplacement :`false` (.x _returnvalue_2)) (select `bool` _bmultiplacement :`false` (.y _returnvalue_2) :`true` (select `bool` (`self.bInvertPlacementDirection`) :`false` _returnvalue_4 :`true` (* _returnvalue_4 -1.0))) 17.0) (`self.K2_GetActorRotation` self)) _returnvalue_3)) (`KismetMathLibrary.MakeRotator` (+ _returnvalue_roll (select `bool` (`self.bInvertPlacementDirection`) :`false` _returnvalue_5 :`true` (* _returnvalue_5 -1.0))) _returnvalue_pitch _returnvalue_yaw)))

(fn `UserConstructionScript`
  (bind _bscalemulticardplacement (`self.bScaleMulticardPlacement`))
  (bind _placementwidth (`self.PlacementWidth`))
  (`|ExecutionSequence`
    (:`then_0`
      (set `self.PlacementWidth` (`KismetMathLibrary.FClamp` (`KismetMathLibrary.GridSnap_Float` (`self.PlacementWidth`) 1.0) 1.0 20.0)))
    (:`then_1`
      (`self.CreateVisualBoardTiles`)
      (`SceneComponent.SetWorldScale3D` (`self.PlacementCollision`) (`KismetMathLibrary.MakeVector` 220.0 (+ (select `bool` _bscalemulticardplacement :`false` 160.0 :`true` (* (/ (`KismetMathLibrary.FClamp` (- _placementwidth 1.0) 1.0 _placementwidth) 2.0) (`self.CardWidth`))) (select `bool` _bscalemulticardplacement :`true` (select `bool` (> _placementwidth 1.0) :`true` 160.0 :!type "Float (single-precision)"))) 5.0)))))