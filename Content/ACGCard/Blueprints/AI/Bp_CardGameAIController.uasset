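; AI controller for the computer opponent in the card game, running behavior tree BT_CardGameAi when it possesses its AI pawn.
; Turn-end events from CardManagerComponent update the blackboard through SetBlackboard, which derives key names from an enum and decodes byte payloads by type.
; AIPlayCard picks a random available placement on the side the card's data allows, calls ServerPlayCard, and returns whether a slot was available.
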(event `self.ReceiveBeginPlay`
  ;[1 1 1] Comment
  (`KismetSystemLibrary.Delay` 2.0)
  (`|ExecutionSequence`
    (:`then_0`
      (bind _ascard_game_state (cast `/Game/ACGCard/Blueprints/CardGameState` (`GameplayStatics.GetGameState`)))
      (set `self.CardGameStateRef` _ascard_game_state))
    (:`then_1`
      (bind _ascard_game_mode (cast `/Game/ACGCard/Blueprints/CardGameMode` (`GameplayStatics.GetGameMode`)))
      (set `self.CardGameModeRef` _ascard_game_mode))))

(event `self.OnPossess`
  (params (PossessedPawn :type "Pawn Object Reference"))
  (bind _asbp_card_game_aipawn (cast `/Game/ACGCard/Blueprints/AI/Bp_CardGameAIPawn` PossessedPawn))
  (set `self.CardGamePawnRef` _asbp_card_game_aipawn)
  (bind _blackboardcomponent (`self.UseBlackboard` "/Game/ACGCard/Blueprints/AI/BB_CardGameAi.BB_CardGameAi"))
  (set `self.AIBlackboardRef` _blackboardcomponent)
  (`self.RunBehaviorTree` "/Game/ACGCard/Blueprints/AI/BT_CardGameAi.BT_CardGameAi")
  (`self.SetDefault`))

(event `self.CardManagerComponent.Server_OnChangeTurnEnd`
  (`self.SetBlackboard` "NewEnumerator6" (`LowEntryExtendedStandardLibrary.BooleanToBytes` (`|EnumEquality` (`/Game/ACGCard/Blueprints/Components/CardManager.TurnState` (`self.CardManagerComponent`)) "NewEnumerator0")))
  (`KismetSystemLibrary.PrintString` "Hello"))

(event `Server_UpdatePlayerState`
  ;[1 1 1] Comment
  (`/Engine/EditorBlueprintResources/ActorMacros.Switch Has Authority`
    (:`Authority`
      (set `/Game/ACGCard/Blueprints/Actor/PlayerDataActor.CardsInHands` (`KismetArrayLibrary.Array_Length` (`/Game/ACGCard/Blueprints/Components/CardManager.CardsInHand` (`self.CardManagerComponent`))) (`/Game/ACGCard/Blueprints/Components/CardManager.PlayerData` (`self.CardManagerComponent`))))))

(fn `AIPlayCard`
  (params (Row :type "DataTableRowHandle Structure") (CardHandIndex :type Integer))
  (returns (Success :type Boolean))
  (bind (_self_player _oppenent) (`/Game/ACGCard/Blueprints/Libs/Misc_FuncLib.GetPlayerIds` self))
  (bind _out_row (`/Game/ACGCard/Blueprints/Libs/Misc_MacroLib.GetRowData` Row))
  (bind (_return_aviableplacement _isaviable) (`/Game/ACGCard/Blueprints/Libs/Cards_FuncLib.GetAviablePlacement` (`/Game/ACGCard/Blueprints/Actor/PlayerDataActor.CardPlacement` (`|GetArrayItem` (`/Game/ACGCard/Blueprints/CardGameState.PlayerDataArray` (`self.CardGameStateRef`)) (select `/Game/ACGCard/Blueprints/Enums/GamePlayEnums/E_Players` (`.Owner_2_E0EDB382468EF502EBD41EA76FA50E7B` (break `/Game/ACGCard/Blueprints/Structs/CardStructs/S_CardPlacement` (`.Placement_28_AF5522054A4BACE33587D196F19C0F73` (break `/Game/ACGCard/Blueprints/Structs/CardStructs/S_Card` _out_row)))) :`NewEnumerator0` _self_player :`NewEnumerator1` _oppenent :`NewEnumerator2` (select `bool` (`KismetMathLibrary.RandomBool`) :`false` _self_player :`true` _oppenent))))))
  (if _isaviable
    (bind _output (`|GetArrayItem` _return_aviableplacement (`KismetMathLibrary.RandomIntegerInRange` 0 (`KismetArrayLibrary.Array_LastIndex` _return_aviableplacement))))
    (bind _returnvalue_location (`KismetMathLibrary.BreakTransform` (`self.GetTransform` _output)))
    (`/Game/ACGCard/Blueprints/Components/CardManager.Server_PlayCard` (`self.CardManagerComponent`) Row _out_row CardHandIndex (`KismetMathLibrary.Conv_VectorToTransform` (`KismetMathLibrary.MakeVector` (.x _returnvalue_location) (.y _returnvalue_location) (+ (.z _returnvalue_location) 100.0))) _output)
    (return true)
    (else
      (return false))))

(fn `SetBlackboard`
  (params (Enum :type "/Game/ACGCard/Blueprints/Enums/AIEnums/E_AIBlackboardKey Enum" :default "NewEnumerator1") (Payload :type "Array of Byte"))
  (bind _aiblackboardref (`self.AIBlackboardRef`))
  (bind _returnvalue (`KismetStringLibrary.Conv_StringToName` (`|GetEnumeratorNameAsString` Enum)))
  (switch `/Game/ACGCard/Blueprints/Enums/AIEnums/E_AIBlackboardKey` Enum
    (:`NewEnumerator1`
      (`BlackboardComponent.SetValueAsFloat` _aiblackboardref _returnvalue (`LowEntryExtendedStandardLibrary.BytesToFloat` Payload)))
    (:`NewEnumerator2`
      (`BlackboardComponent.SetValueAsEnum` _aiblackboardref _returnvalue (`LowEntryExtendedStandardLibrary.BytesToByte` Payload) :!label _label))
    (:`NewEnumerator3`
      (goto _label))
    (:`NewEnumerator4`
      (`BlackboardComponent.SetValueAsInt` _aiblackboardref _returnvalue (`LowEntryExtendedStandardLibrary.BytesToInteger` Payload) :!label _label_2))
    (:`NewEnumerator5`
      (goto _label_2))
    (:`NewEnumerator6`
      (`BlackboardComponent.SetValueAsBool` _aiblackboardref _returnvalue (`LowEntryExtendedStandardLibrary.BytesToBoolean` Payload) :!label _label_3))
    (:`NewEnumerator7`
      (goto _label_3))
    (:`NewEnumerator8`
      (goto _label_3))
    (:`NewEnumerator9`
      (goto _label_3))))

(fn `SetDefault`
  (`self.SetBlackboard` "NewEnumerator3" (`LowEntryExtendedStandardLibrary.ByteToBytes` (enumliteral `/Game/ACGCard/Blueprints/Enums/AIEnums/E_AITurnState` "NewEnumerator0")))
  (`self.SetBlackboard` "NewEnumerator1" (`LowEntryExtendedStandardLibrary.FloatToBytes` 2.0)))

(fn `UpdateAIState`
  (`/Engine/EditorBlueprintResources/ActorMacros.Switch Has Authority`))

(fn `UserConstructionScript`)