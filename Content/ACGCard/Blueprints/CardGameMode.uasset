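; Game mode for the card game that registers players on login and starts the match once all seats are filled.
; Outside MainMenu, the server's PostLogin records card player controllers, indexes BoardPlayer actors by PlayerIndex and checks the player count.
; A full roster sets GameActive and emits a state enum through CardGameState.
; ForceSpawnAIOpponent spawns AI pawns at the next free board position, adds their controllers and starts the game directly.
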(event `self.ReceiveBeginPlay`
  ;[1 1 1] Comment
  (`KismetSystemLibrary.Delay` 0.2)
  (`|ExecutionSequence`
    (:`then_0`
      (bind _ascard_game_state (cast `/Game/ACGCard/Blueprints/CardGameState` (`GameplayStatics.GetGameState`)))
      (set `self.GameStateRef` _ascard_game_state))
    (:`then_1`
      (cast `/Game/ACGCard/Blueprints/CardGameInstance` (`GameplayStatics.GetGameInstance`)))))

(event `self.K2_PostLogin`
  (params (NewPlayer :type "PlayerController Object Reference"))
  (bind (_ascard_game_player_controller _bsuccess) (cast `/Game/ACGCard/Blueprints/CardGamePlayerController` NewPlayer :!pure true))
  ;[1 1 1] SetupPlayer
  (`/Engine/EditorBlueprintResources/ActorMacros.Switch Has Authority`
    (:`Authority`
      (bind _returnvalue (`GameplayStatics.GetCurrentLevelName` true))
      (if (not (`KismetStringLibrary.EqualEqual_StrStr` _returnvalue "MainMenu"))
        (if (>= (`KismetArrayLibrary.Array_Length` (`self.GameControllersArray`)) (`self.MaxNumOfPlayers`))
          (`self.SetBoardPlayer` :!label _label)
          (elif _bsuccess
            (`KismetArrayLibrary.Array_AddUnique` (`self.GameControllersArray`) _ascard_game_player_controller)
            (`self.SetBoardPlayer`)
            (`/Game/ACGCard/Blueprints/CardGamePlayerController.Client_Post  Login` _ascard_game_player_controller)
            (else
              (goto _label))))
        (`self.CheckGamePreconditions`)))))

(event `CheckGamePreconditions`
  ;[1 1 1] Check Game Preconditions
  (`/Engine/EditorBlueprintResources/ActorMacros.Switch Has Authority`
    (:`Authority`
      (if (== (`KismetArrayLibrary.Array_Length` (`self.GameControllersArray`)) (`self.MaxNumOfPlayers`))
        (`KismetSystemLibrary.PrintString` "All players are in!" true true (struct :`R` 0.03415 :`G` 1.0 :`A` 1.0) 10.0 :!label _label_2)
        (set `self.bGameActive` true)
        (`/Game/ACGCard/Blueprints/CardGameState.EmitEnum` (`self.GameStateRef`) "NewEnumerator3")))))

(event `ForceSpawnAIOpponent`
  ;[1 1 1] Check Game Preconditions
  (`self.CreateAIOpponent`)
  (goto _label_2))

(fn `CreateAIOpponent`
  (if (< (`KismetArrayLibrary.Array_Length` (`self.GameControllersArray`)) (`self.MaxNumOfPlayers`))
    (for _ (range 1 3)
      (bind _returnvalue (`AIBlueprintHelperLibrary.SpawnAIFromClass` "/Game/ACGCard/Blueprints/AI/Bp_CardGameAIPawn.Bp_CardGameAIPawn_C" null (`self.K2_GetActorLocation` (`|GetArrayItem` (`self.BoardPlayersArray`) (`KismetArrayLibrary.Array_Length` (`self.GameControllersArray`)))) (struct) true))
      (`KismetArrayLibrary.Array_AddUnique` (`self.GameControllersArray`) (`Pawn.GetController` _returnvalue)))))

(fn `HandlePlayer`
  (params (PlayerController :type "/Game/ACGCard/Blueprints/CardGamePlayerController Object Reference (by ref)") (PlayerState :type "/Game/ACGCard/Blueprints/CardGamePlayerState Object Reference")))

(fn `OnRep_GameControllersArray`)

(fn `SetBoardPlayer`
  (bind _outactors (`GameplayStatics.GetAllActorsOfClass` "/Game/ACGCard/Blueprints/GamePlay/BoardPlayer.BoardPlayer_C"))
  (for _array_element _outactors
    (`KismetArrayLibrary.Array_Set` (`self.BoardPlayersArray`) (`/Game/ACGCard/Blueprints/GamePlay/BoardPlayer.PlayerIndex` _array_element) _array_element true)))

(fn `UserConstructionScript`)