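; Player controller for a networked card game, handling card drag-and-drop, game UI, turn-change requests and AI opponent spawning.
; On the active turn, a client-side preview card follows the pointer with interpolation while placements are validated by owner.
; Valid drops go to the server, which charges mana, removes the hand card and spawns the real card; board assignment is an empty stub.
; CardManagerComponent events and client calls refresh the hand and opponent UI.
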(event `Bind Event`
  ;[1 1 1] c
  (add `self.EmitPlayerState` (delegate `EmitPlayerState_Event`)))

(event `EmitPlayerState_Event` :!signature `self.EmitPlayerState`
  (params (PlayerState :type "/Game/ACGCard/Blueprints/Enums/GamePlayEnums/E_PlayerState Enum" :default "NewEnumerator0"))
  ;[1 1 1] c
  (set `self.PlayerStateEnum` PlayerState))

(event `self.ReceiveBeginPlay`
  ;[1 1 1] Comment
  (`|ExecutionSequence`
    (:`then_0`
      (`|ExecutionSequence`
        (:`then_0`
          (bind _ascard_game_mode (cast `/Game/ACGCard/Blueprints/CardGameMode` (`GameplayStatics.GetGameMode`)))
          (set `self.CardGameModeRef` _ascard_game_mode))
        (:`then_1`
          (bind _ascard_game_state (cast `/Game/ACGCard/Blueprints/CardGameState` (`GameplayStatics.GetGameState`)))
          (set `self.CardGameStateRef` _ascard_game_state))))
    (:`then_1`
      (`/Engine/EditorBlueprintResources/ActorMacros.Switch Has Authority`
        (:`Authority`
          (`self.Bind Event`))))
    (:`then_3`
      (`WidgetBlueprintLibrary.SetInputMode_GameAndUIEx` self null "DoNotLock" false))))

(event `InputTouch`
  (params (Location :type "Vector Structure") (FingerIndex :type "ETouchIndex Enum"))
  (bind _playerstateenum (`self.PlayerStateEnum`))
  (:`Released`
    (`self.IsTurnActive` :!label _label
      (:`true`
        (switch `/Game/ACGCard/Blueprints/Enums/GamePlayEnums/E_PlayerState` _playerstateenum
          (:`NewEnumerator2`
            (if (`self.bIsValidClientDrop`)
              (`self.Server_PlayCard` (`self.TempCardRow`) (`self.TempHandIndex`) (`self.GetTransform` (`self.PlayCard_Client_Ref`)))
              (else
                (`self.Client_DropCard`)
                (`self.K2_DestroyActor` (`self.PlayCard_Client_Ref`) :!label _label_2)
                (set `self.PlayCard_Client_Ref` null)))
            (set `self.PlayerStateEnum` "NewEnumerator0"))))))
  (:`Moved`
    (`self.IsTurnActive`
      (:`true`
        (switch `/Game/ACGCard/Blueprints/Enums/GamePlayEnums/E_PlayerState` _playerstateenum :!label _label_3
          (:`NewEnumerator2`
            (`self.SetCardLocation` (`/Game/ACGCard/Blueprints/Libs/Misc_FuncLib.MouseDistanceInWorldSpace` self (`self.CardHoldDistance`)) (`self.PlayCard_Client_Ref`) (`/Game/ACGCard/Blueprints/Libs/Misc_FuncLib.GetWorldRotationForPlayer` (struct)))
            (`self.ValidateCardPlacement` (`/Game/ACGCard/Blueprints/Libs/Misc_FuncLib.MouseToWorldLocation` self))
            (`KismetSystemLibrary.Delay` 0.01)
            (goto _label_3)))))))

(event `Client_Post  Login`
  ;[1 1 1] Clent Post Login
  (`KismetSystemLibrary.Delay` 1.0) ; This short delay helps stop referencing actors that might not yet be available.
  (`self.SetupGameUI`))

(event `OnDragCancle`
  (goto _label))

(event `DestroyClientCard`
  (goto _label_2))

(event `self.CardManagerComponent.UpdateUI`
  ;[1 1 1] Comment
  (`self.Update GameUI`))

(event `Key|LeftMouseButton`
  (params (Key :type "Key Structure"))
  (:`Pressed`
    (goto _label))
  (:`Released`
    (goto _label)))

(event `self.CardManagerComponent.DrawCardEnd`
  (params (Card :type "DataTableRowHandle Structure"))
  ;[1 1 1] Comment
  (`self.Client Add Card` Card))

(event `Spawn AI Oppenent`
  ;[1 1 1] Comment
  (bind _ascard_game_mode (cast `/Game/ACGCard/Blueprints/CardGameMode` (`GameplayStatics.GetGameMode`)))
  (`/Game/ACGCard/Blueprints/CardGameMode.ForceSpawnAIOpponent` _ascard_game_mode))

(event `Server_ChangeTurn`
  (bind _cardgamestateref (`self.CardGameStateRef`))
  ;[1 1 1] Comment
  (if (`/Game/ACGCard/Blueprints/CardGameState.RequestChangeTurn` _cardgamestateref self)
    (`/Game/ACGCard/Blueprints/CardGameState.Server_RequestChangeTurnState` _cardgamestateref self)))

(event `Server_PlayCard`
  (params (Row :type "DataTableRowHandle Structure") (CardHandIndex :type Integer) (SpawnTransform :type "Transform Structure"))
  (`self.PlayCard` Row CardHandIndex SpawnTransform))

(event `Update GameUI`
  ;[1 1 1] Comment
  (`/Engine/EditorBlueprintResources/StandardMacros.IsValid` (`self.PlayerGameUI`)
    (:`Is Valid`
      (`/Game/ACGCard/Blueprints/Widgets/GamePlay/W_OpponentUI.Client_UpdateUI_Event_0` (`/Game/ACGCard/Blueprints/Widgets/GamePlay/W_PlayerGameUI.W_OpponentUI` (`self.PlayerGameUI`))))))

(event `Client Add Card`
  (params (Cards :type "DataTableRowHandle Structure"))
  (bind _playergameui (`self.PlayerGameUI`))
  ;[1 1 1] Comment
  (`/Engine/EditorBlueprintResources/StandardMacros.IsValid` _playergameui
    (:`Is Valid`
      (`/Game/ACGCard/Blueprints/Widgets/GamePlay/W_CardManager.Client_AddCard` (`/Game/ACGCard/Blueprints/Widgets/GamePlay/W_PlayerGameUI.W_CardManager` _playergameui) Cards))))

(event `Client_RemoveCardFromCardManager`
  (params (CardToRemove :type "/Game/ACGCard/Blueprints/Widgets/GamePlay/W_CardWidget Object Reference") (index :type Integer))
  ;[1 1 1] Comment
  (`/Game/ACGCard/Blueprints/Widgets/GamePlay/W_CardManager.RemoveCardFromHand` (`/Game/ACGCard/Blueprints/Widgets/GamePlay/W_PlayerGameUI.W_CardManager` (`self.PlayerGameUI`)) CardToRemove index))

(event `Client_DropCard`
  (bind _asw_card_widget (cast `/Game/ACGCard/Blueprints/Widgets/GamePlay/W_CardWidget` (`DragDropOperation.Payload` (`self.DragDrop Operation Ref`))))
  (`/Game/ACGCard/Blueprints/Widgets/GamePlay/W_CardWidget.Set Default` _asw_card_widget))

(event `Call Create Card`
  (params (`DragDrop Operation Ref` :type "DragDropOperation Object Reference") (TempHandIndex :type Integer) (Row :type "DataTableRowHandle Structure"))
  ;[1 1 1] Comment
  (`self.IsTurnActive`
    (:`true`
      (set `self.DragDrop Operation Ref` `DragDrop Operation Ref`)
      (set `self.TempHandIndex` TempHandIndex)
      (set `self.TempCardRow` Row)
      (set `self.PlayerStateEnum` "NewEnumerator2")
      (`self.CreatePlaceableCard(Client)` (`/Game/ACGCard/Blueprints/Libs/Misc_FuncLib.MouseDistanceInWorldSpace` self 1500.0) Row))))

(event `PlayCard`
  (params (Row :type "DataTableRowHandle Structure") (CardHandIndex :type Integer) (SpawnTransform :type "Transform Structure") (CardPlacement :type "/Game/ACGCard/Blueprints/GamePlay/CardPlacement Object Reference"))
  (bind _cardmanagercomponent (`self.CardManagerComponent`))
  ;[1 1 1] Comment
  (`/Engine/EditorBlueprintResources/ActorMacros.Switch Has Authority`
    (:`Authority`
      (bind _out_row (`/Game/ACGCard/Blueprints/Libs/Misc_MacroLib.GetRowData` Row))
      (bind _valid (`/Game/ACGCard/Blueprints/Components/CardManagerComponent.ChargeManaCost` _cardmanagercomponent _out_row))
      (if _valid
        (`self.RemoveCardFromHand` Row CardHandIndex)
        (bind _output_get (`self.CreatePlaceableCard(Server)` SpawnTransform))
        (`/Game/ACGCard/Blueprints/GamePlay/Card.Server_SetupCard` _output_get _out_row)
        (`self.AddCardToBoardPlacement` _output_get CardPlacement (`/Game/ACGCard/Blueprints/Components/CardManagerComponent.PlayerId` (`self.CardManagerComponent`)))
        (else
          (`/Game/ACGCard/Blueprints/Components/CardManagerComponent.EmitCardMessage` _cardmanagercomponent "NewEnumerator1")))
      (`self.DestroyClientCard`)
      (`self.Client_DropCard`)
      (`/Game/ACGCard/Blueprints/Components/CardManagerComponent.Server_UpdatePlayerState` (`self.CardManagerComponent`)))))

(fn `AddCardToBoardPlacement`
  (params (Card :type "/Game/ACGCard/Blueprints/GamePlay/Card Object Reference") (GoalBoard :type "/Game/ACGCard/Blueprints/GamePlay/CardPlacement Object Reference") (OwnPlayerID :type Integer)))

(fn `CreatePlaceableCard(Client)`
  (params (`Spawn Transform Location` :type "Vector Structure") (Row :type "DataTableRowHandle Structure"))
  (bind _returnvalue (`|SpawnActorFromClass` "/Game/ACGCard/Blueprints/GamePlay/Card.Card_C" (`KismetMathLibrary.MakeTransform` `Spawn Transform Location` (`/Game/ACGCard/Blueprints/Libs/Misc_FuncLib.GetWorldRotationForPlayer` (struct))) "Undefined" "OverrideRootScale" self null))
  (set `self.PlayCard_Client_Ref` _returnvalue)
  (return))

(fn `CreatePlaceableCard(Server)`
  (params (SpawnTransform :type "Transform Structure"))
  (returns (Output_Get :type "/Game/ACGCard/Blueprints/GamePlay/Card Object Reference"))
  (`/Engine/EditorBlueprintResources/ActorMacros.Switch Has Authority`
    (:`Authority`
      (set `self.TEMP_SpawnTransform` SpawnTransform)
      (bind _returnvalue (`|SpawnActorFromClass` "/Game/ACGCard/Blueprints/GamePlay/Card.Card_C" SpawnTransform "Undefined" "OverrideRootScale" self null))
      (bind _output_get (set `self.PlayCard_Server_Ref` _returnvalue))
      (return _output_get))
    (:`Remote`
      (return null))))

(fn `RemoveCardFromHand`
  (params (Row :type "DataTableRowHandle Structure") (Index :type Integer))
  (returns (Success :type Boolean))
  (bind _cardsinhand (`/Game/ACGCard/Blueprints/Components/CardManagerComponent.CardsInHand` (`self.CardManagerComponent`)))
  (`/Engine/EditorBlueprintResources/ActorMacros.Switch Has Authority`
    (:`Authority`
      (if (`/Game/ACGCard/Blueprints/Libs/Misc_FuncLib.CompareRow` Row (`|GetArrayItem` _cardsinhand Index))
        (`KismetArrayLibrary.Array_Remove` _cardsinhand Index)
        (`self.Client_RemoveCardFromCardManager` null Index)
        (`/Game/ACGCard/Blueprints/Components/CardManagerComponent.Server_UpdatePlayerState` (`self.CardManagerComponent`))
        (return true)
        (else
          (return false))))))

(fn `SetCardLocation`
  (params (HoldLocation :type "Vector Structure") (Card :type "/Game/ACGCard/Blueprints/GamePlay/Card Object Reference") (Rotation :type "Rotator Structure"))
  (bind _returnvalue (`GameplayStatics.GetWorldDeltaSeconds`))
  (bind _returnvalue_2 (`self.K2_GetActorLocation` Card))
  (bind _yaw (.yaw Rotation))
  (bind _returnvalue_3 (> _yaw 0.0))
  (bind _returnvalue_4 (/ (- (.x _returnvalue_2) (.x HoldLocation)) 5.0))
  (bind _returnvalue_5 (/ (- (.y _returnvalue_2) (.y HoldLocation)) 5.0))
  (`/Engine/EditorBlueprintResources/StandardMacros.IsValid` Card
    (:`Is Valid`
      (`self.K2_SetActorLocation` Card (`KismetMathLibrary.VInterpTo` _returnvalue_2 HoldLocation _returnvalue 10.0) false false) ; Set the Card in hand's location
      (if (`self.bEnableInHandMovementRotation`)
        (`self.K2_SetActorRotation` Card (`KismetMathLibrary.RInterpTo` (`self.K2_GetActorRotation` Card) (`KismetMathLibrary.MakeRotator` (select `bool` _returnvalue_3 :`false` _returnvalue_5 :`true` (* _returnvalue_5 -1.0)) (select `bool` _returnvalue_3 :`false` (* _returnvalue_4 -1.0) :`true` _returnvalue_4) _yaw) _returnvalue 5.0) false) ; Sets rotation of the card based on the movement speed of the mouse.
      ))
    (:`Is Not Valid`
      _))
  (return))

(fn `SetupGameUI`
  (if (`self.IsLocalPlayerController`)
    (bind _returnvalue (`|CreateWidget` "/Game/ACGCard/Blueprints/Widgets/GamePlay/W_PlayerGameUI.W_PlayerGameUI_C" self))
    (bind _output_get (set `self.PlayerGameUI` _returnvalue))
    (`UserWidget.AddToViewport` _output_get 2))
  (return))

(fn `UserConstructionScript`)

(fn `ValidateCardPlacement`
  (params (`Hit Actor` :type "Actor Object Reference"))
  (returns (Output_Get :type Boolean))
  (bind _targetcardplacement (`self.TargetCardPlacement`))
  (bind _cardplacement (`self.CardPlacement`))
  (bind _output_get (set `self.HitActor` `Hit Actor`))
  (bind _ascard_placement (cast `/Game/ACGCard/Blueprints/GamePlay/CardPlacement` _output_get)
    (:`then`
      (if (not (== _ascard_placement (`self.TargetCardPlacement`)))
        (bind _output_get_2 (set `self.CardPlacement` _ascard_placement))
        (bind _out_row (`/Game/ACGCard/Blueprints/Libs/Misc_MacroLib.GetRowData` (`self.TempCardRow`)))
        (`self.ValidatePlacementOwner` (`/Game/ACGCard/Blueprints/Components/CardManagerComponent.PlayerId` (`self.CardManagerComponent`)) (`/Game/ACGCard/Blueprints/GamePlay/CardPlacement.PlayerId` _output_get_2) _out_row
          (:`Both`
            (`/Engine/EditorBlueprintResources/StandardMacros.IsValid` _targetcardplacement :!label _label
              (:`Is Valid`
                (if (not (== _targetcardplacement _cardplacement))
                  (set `self.TargetCardPlacement` _cardplacement :!label _label_2)))
              (:`Is Not Valid`
                (goto _label_2)))
            (bind _output_get_3 (set `self.bIsValidClientDrop` true)))
          (:`Self`
            (goto _label))
          (:`Oppenent`
            (goto _label))
          (:`None`
            (set `self.CardPlacement` null :!label _label_3)
            (set `self.TargetCardPlacement` null)
            (set `self.bIsValidClientDrop` false)))))
    (:`CastFailed`
      (cast `/Game/ACGCard/Blueprints/GamePlay/Card` _output_get
        (:`CastFailed`
          (goto _label_3)))))
  (return _output_get_3))