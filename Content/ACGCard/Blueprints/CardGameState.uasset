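; Game state for a card game that handles match start and the initial card deal on the server.
; On BeginPlay it caches the game mode, loads the default card table as row handles and listens to ServerInteractionComponent enum events.
; Game Start sets game and turn timers, then gives each controller's CardManagerComponent random cards and a PlayerId.
; A delayed debug call targets game start; turn-order logic is unwired, with empty begin/end turn stubs.
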(event `self.ReceiveBeginPlay`
  (bind _defaultcardtable (`self.DefaultCardTable`))
  (`/Engine/EditorBlueprintResources/ActorMacros.Switch Has Authority`
    (:`Authority`
      (`|ExecutionSequence`
        (:`then_0`
          (`KismetSystemLibrary.Delay` 0.2)
          (bind _ascard_game_mode (cast `/Game/ACGCard/Blueprints/CardGameMode` (`GameplayStatics.GetGameMode`))
            (:`then`
              (set `self.CardGameModeRef` _ascard_game_mode))
            (:`CastFailed`
              (`KismetSystemLibrary.PrintString` "Game Mode Cast Failed"))))
        (:`then_1`
          (bind _outrownames (`DataTableFunctionLibrary.GetDataTableRowNames` _defaultcardtable))
          (for _array_element _outrownames
            (`KismetArrayLibrary.Array_Add` (`self.DefaultCard`) (make `DataTableRowHandle` _defaultcardtable _array_element))))
        (:`then_2`
          (`self.Bind Event`))
        (:`then_3`
          ;[1 0.05451 0 0.298] Development
          (`KismetSystemLibrary.Delay` 2.0)
          (`self.Debug_GameStart`))))))

(event `Bind Event`
  (add `/Game/ACGCard/Blueprints/Components/InteractionComponent.EmitEnumV1` (`self.ServerInteractionComponent`) (delegate `EmitEnumV1_Event_0`)))

(event `EmitEnumV1_Event_0`
  (params (InteractionKey :type "/Game/ACGCard/Blueprints/Enums/InteractionEnum/E_InteractionV1 Enum" :default "NewEnumerator0") (Value :type Byte))
  (bind _cardgamemoderef (`self.CardGameModeRef`))
  (bind _gameseconds (`/Game/ACGCard/Blueprints/CardGameMode.GameSeconds` _cardgamemoderef))
  (switch `/Game/ACGCard/Blueprints/Enums/InteractionEnum/E_InteractionV1` InteractionKey
    (:`NewEnumerator1`
      (switch `/Game/ACGCard/Blueprints/Enums/InteractionEnum/E_GameStateV1` (cast `/Game/ACGCard/Blueprints/Enums/InteractionEnum/E_GameStateV1` Value)
        (:`NewEnumerator3`
          (`|ExecutionSequence`
            (:`then_0`
              (set `self.GameControllerArray` (`/Game/ACGCard/Blueprints/CardGameMode.GameControllersArray` _cardgamemoderef))
              (bind _returnvalue (`KismetSystemLibrary.K2_SetTimer` null "GameTimer" _gameseconds))
              (set `self.GameTimerRef` _returnvalue)
              (bind _returnvalue_2 (`KismetSystemLibrary.K2_SetTimer` null "TurnTimer" _gameseconds true))
              (set `self.TurnTimerRef` _returnvalue_2))
            (:`then_1`
              (for (_array_element _array_index) (`self.GameControllerArray`)
                (bind _variable (`/Game/ACGCard/Blueprints/Libs/Misc_MacroLib.GetRandItemsArray` (`self.DefaultCard`) (`self.NumberOfCardNeedPickup`))
                  (:`Completed`
                    (`|ExecutionSequence`
                      (:`then_0`
                        (bind _returnvalue_3 (`self.GetComponentByClass` _array_element "/Game/ACGCard/Blueprints/Components/CardManagerComponent.CardManagerComponent_C"))
                        (`/Game/ACGCard/Blueprints/Components/CardManagerComponent.AddCard` _returnvalue_3 _variable)
                        (set `/Game/ACGCard/Blueprints/Components/CardManagerComponent.PlayerId` _array_index _returnvalue_3)))))))))))))

(event `Debug_GameStart`
  ;[1 0.05451 0 0.298] Development
  (`/Game/ACGCard/Blueprints/Components/InteractionComponent.EmitEnumV1` (`self.ServerInteractionComponent`) "NewEnumerator1" (enumliteral `/Game/ACGCard/Blueprints/Enums/InteractionEnum/E_GameStateV1` "NewEnumerator3")))

(fn `BeginPlayerTurn`
  (params (Id :type Integer)))

(fn `EndPlayerTurn`
  (params (Id :type Integer)))

(fn `Reset Turn Time`
  (set `self.TurnTime_Seconds` (`self.TurnDuration_Seconds`))
  (set `self.TurnTime_Minutes` (`self.TurnDuration_Minutes`)))

(fn `UserConstructionScript`)