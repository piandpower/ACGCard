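; Replicated per-player data actor for the card game, tracking health, mana, turn, hand count and active card controls.
; On the server, BeginPlay initializes stats from CardGameMode and binds update dispatchers from CardManager and itself.
; These key-based updates refresh the hand count and recompute the attackable card list.
; OnRep functions for mana and hand count notify clients through a matching replication dispatcher.
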(event `self.ReceiveBeginPlay`
  (`/Engine/EditorBlueprintResources/ActorMacros.Switch Has Authority`
    (:`Authority`
      (`|ExecutionSequence`
        (:`then_0`
          (`|ExecutionSequence`
            (:`then_0`
              (bind _ascard_game_mode (cast `/Game/ACGCard/Blueprints/CardGameMode` (`GameplayStatics.GetGameMode`)))
              (set `self.CardGameMode` _ascard_game_mode))))
        (:`then_1`
          (`self.InitAttribute`))
        (:`then_2`
          (add `/Game/ACGCard/Blueprints/Components/CardManager.Server_UpdateReplication` (`self.CardManager`) (delegate `Server_UpdateReplication_Event_0`))
          (add `self.Server_UpdateReplication` (delegate `Server_UpdateReplication_Event`)))))))

(event `Server_UpdateReplication_Event_0`
  (params (Replication :type "/Game/ACGCard/Blueprints/Enums/ReplicationEnum/E_CardManagerReplication Enum" :default "NewEnumerator0"))
  (switch `/Game/ACGCard/Blueprints/Enums/ReplicationEnum/E_CardManagerReplication` Replication
    (:`NewEnumerator1`
      (set `self.CardsInHands` (`KismetArrayLibrary.Array_Length` (`/Game/ACGCard/Blueprints/Components/CardManager.CardStructInHand` (`self.CardManager`)))))))

(event `Server_UpdateReplication_Event` :!signature `self.Server_UpdateReplication`
  (params (Replication :type "/Game/ACGCard/Blueprints/Enums/ReplicationEnum/E_PlayerDataReplication Enum" :default "NewEnumerator0"))
  (switch `/Game/ACGCard/Blueprints/Enums/ReplicationEnum/E_PlayerDataReplication` Replication
    (:`NewEnumerator6`
      (set `self.AttackAbleList` (`/Game/ACGCard/Blueprints/Libs/Cards_FuncLib.FilterAttackAbleCard` (`self.ActiveCardControl`))))))

(event `ServerEvent_UpdateReplication`
  (params (Key :type "/Game/ACGCard/Blueprints/Enums/ReplicationEnum/E_PlayerDataReplication Enum" :default "NewEnumerator0"))
  (`self.Server_UpdateReplication` Key))

(fn `DecreaseMana`
  (params (value :type Integer))
  (`/Engine/EditorBlueprintResources/ActorMacros.Switch Has Authority`
    (:`Authority`
      (set `self.Mana` (`KismetMathLibrary.Clamp` (- (`self.Mana`) value) 0 (`self.ManaMax`)))
      (return))))

(fn `GetManaForTurn`
  (returns (Mana :type Integer))
  (bind _mana (`/Game/ACGCard/Blueprints/CardGameMode.CaculateManaForTurn` (`self.CardGameMode`) (`self.PlayerTurn`)))
  (bind _output_get (set `self.Mana` _mana))
  (return _output_get))

(fn `InitAttribute`
  (`/Engine/EditorBlueprintResources/ActorMacros.Switch Has Authority`
    (:`Authority`
      (set `self.Health` (`/Game/ACGCard/Blueprints/CardGameMode.PlayerStartHealth` (`self.CardGameMode`)))
      (set `self.Mana` 0)
      (`self.SetCardControl` (`/Game/ACGCard/Blueprints/GamePlay/BoardPlayer.CardConrol` (`/Game/ACGCard/Blueprints/Components/CardManager.BoardPlayerRef` (`self.CardManager`)))))))

(fn `OnRep_CardsInHands`
  (`self.Client_UpdateReplication` "NewEnumerator4"))

(fn `OnRep_Health`)

(fn `OnRep_Mana`
  (`self.Client_UpdateReplication` "NewEnumerator3"))

(fn `OnRep_PlayerTurn`)

(fn `SetCardControl`
  (params (CardControl :type "/Game/ACGCard/Blueprints/Components/CardControl Object Reference") (`IsRemove?` :type Boolean))
  (bind _activecardcontrol (`self.ActiveCardControl`))
  (`/Engine/EditorBlueprintResources/ActorMacros.Switch Has Authority`
    (:`Authority`
      (if `IsRemove?`
        (`KismetArrayLibrary.Array_RemoveItem` _activecardcontrol CardControl)
        (else
          (`KismetArrayLibrary.Array_AddUnique` _activecardcontrol CardControl)))
      (`self.ServerEvent_UpdateReplication` "NewEnumerator6"))))

(fn `UserConstructionScript`)