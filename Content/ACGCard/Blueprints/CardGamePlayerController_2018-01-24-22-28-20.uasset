(event `Call Create Card`
  (params (`DragDrop Operation Ref` :type "DragDropOperation Object Reference") (TempHandIndex :type Integer) (TempCardStruct :type "/Game/ACGCard/Blueprints/Structs/CardStructs/S_Card Structure"))
  ;[1 1 1] Comment
  (`self.IsTurnActive`
    (:`true`
      (`|ExecutionSequence`
        (:`then_0`
          (set `self.DragDrop Operation Ref` `DragDrop Operation Ref`)
          (set `self.TempHandIndex` TempHandIndex)
          (set `self.PlayerStateEnum` "NewEnumerator2")
          (bind _output_get (set `self.TempCardStruct` TempCardStruct)))
        (:`then_1`
          (bind _returnvalue (`|SpawnActorFromClass` "/Game/ACGCard/Blueprints/GamePlay/Card.Card_C" (`KismetMathLibrary.MakeTransform` (`/Game/ACGCard/Blueprints/Libs/Misc_FuncLib.MouseDistanceInWorldSpace` self 1500.0) (`/Game/ACGCard/Blueprints/Libs/Misc_FuncLib.GetWorldRotationForPlayer` (struct))) "Undefined" "OverrideRootScale" self null 0 _output_get null))
          (set `self.PlayCard_Client_Ref` _returnvalue)
          (`/Game/ACGCard/Blueprints/GamePlay/Card.SetCardVisual` _returnvalue))))))

(event `self.ReceiveBeginPlay`
  ;[1 1 1] Comment
  (`KismetSystemLibrary.Delay` 2.0)
  (if (`self.IsLocalPlayerController`)
    (`|ExecutionSequence`
      (:`then_0`
        (`self.InitVariable`))
      (:`then_1`
        (`WidgetBlueprintLibrary.SetInputMode_GameAndUIEx` self null "DoNotLock" false)))))

(event `InputTouch`
  (params (Location :type "Vector Structure") (FingerIndex :type "ETouchIndex Enum"))
  (bind _playerstateenum (`self.PlayerStateEnum`))
  ;[1 1 1] Comment
  (:`Pressed`
    (`self.IsTurnActive`
      (:`true`
        (`self.DetectCardInteraction`))))
  (:`Released`
    (`self.IsTurnActive` :!label _label
      (:`true`
        (switch `/Game/ACGCard/Blueprints/Enums/GamePlayEnums/E_PlayerState` _playerstateenum
          (:`NewEnumerator1`
            (bind _bvalidinteraction (`self.ValidateInteractionState`))
            (if _bvalidinteraction
              (`/Game/ACGCard/Blueprints/Components/CardManager.Server_RunCardInteraction` (`self.CardManagerComponent`) (`self.TakingControl`) (`self.RecevingControl`)))
            (`self.CleanCardInteraction`)
            (`self.SetCardInteraction` "NewEnumerator0"))
          (:`NewEnumerator2`
            (`self.CleanCardPlacement`)
            (if (`self.bIsValidClientDrop`)
              (`/Game/ACGCard/Blueprints/Libs/Card_MacroLib.ServerPlaceCard` (`self.CardManagerComponent`) (`self.TempCardStruct`) (`self.GetTransform` (`self.PlayCard_Client_Ref`)) (`self.TargetCardPlacement`) (`self.TempHandIndex`) (`self.TempInsertIndex`)
                (:`Success`
                  _)
                (:`Falid`
                  _)))
            (`self.Client_DropCard`)
            (`self.K2_DestroyActor` (`self.PlayCard_Client_Ref`) :!label _label_2)
            (set `self.PlayCard_Client_Ref` null)
            (set `self.PlayerStateEnum` "NewEnumerator0"))))))
  (:`Moved`
    (`self.IsTurnActive`
      (:`true`
        (`|ExecutionSequence`
          (:`then_0`
            (switch `/Game/ACGCard/Blueprints/Enums/GamePlayEnums/E_PlayerState` _playerstateenum
              (:`NewEnumerator1`
                (`self.DetectCardInteractionOnMove`))
              (:`NewEnumerator2`
                (`self.SetCardLocation` (`/Game/ACGCard/Blueprints/Libs/Misc_FuncLib.MouseDistanceInWorldSpace` self (`self.CardHoldDistance`)) (`self.PlayCard_Client_Ref`) (`/Game/ACGCard/Blueprints/Libs/Misc_FuncLib.GetWorldRotationForPlayer` (struct)))
                (`self.ValidateCardPlacementOnMove` (`/Game/ACGCard/Blueprints/Libs/Misc_FuncLib.MouseToWorldLocation` self))
                (`KismetSystemLibrary.Delay` 0.01))))
          (:`then_1`
            (goto _label_3 :!via `Reset`))))
      (:`false`
        (`/Engine/EditorBlueprintResources/StandardMacros.DoOnce` false :!label _label_3
          (:`Completed`
            (`self.CleanCardPlcamentState`
              (:`out`
                (`self.CleanCardInteraction`)))))))))

(event `Client_Post  Login`
  ;[1 1 1] Clent Post Login
  (`KismetSystemLibrary.Delay` 1.0) ; This short delay helps stop referencing actors that might not yet be available.
  (`self.SetupGameUI`))

(event `OnDragCancle`
  ;[1 1 1] Comment
  (goto _label))

(event `Key|LeftMouseButton`
  (params (Key :type "Key Structure"))
  ;[1 1 1] Comment
  (:`Released`
    (goto _label)))

(event `Spawn Ai Oppent`
  (bind _ascard_game_mode (cast `/Game/ACGCard/Blueprints/CardGameMode` (`GameplayStatics.GetGameMode`)))
  (`/Game/ACGCard/Blueprints/CardGameMode.ForceSpawnAIOpponent` _ascard_game_mode))

(event `DestroyClientCard`
  ;[1 1 1] Comment
  (goto _label_2))

(event `Client_DropCard`
  ;[1 1 1] Comment
  (bind _asw_card_widget (cast `/Game/ACGCard/Blueprints/Widgets/GamePlay/W_CardWidget` (`DragDropOperation.Payload` (`self.DragDrop Operation Ref`))))
  (`/Game/ACGCard/Blueprints/Widgets/GamePlay/W_CardWidget.Set Default` _asw_card_widget)
  (set `/Game/ACGCard/Blueprints/Widgets/GamePlay/W_CardManager.IsDrag` false (`/Game/ACGCard/Blueprints/Widgets/GamePlay/W_PlayerGameUI.W_CardManager` (`self.PlayerGameUI`))))

(event `Client_MouseOverCard`
  (params (Card :type "/Game/ACGCard/Blueprints/GamePlay/Card Object Reference") (IsOver :type Boolean))
  (bind _viewcardpreview (`self.ViewCardPreview`))
  (if IsOver
    (`/Game/ACGCard/Blueprints/Widgets/GamePlay/W_CardPreview.InitialCardPreview` _viewcardpreview (`/Game/ACGCard/Blueprints/GamePlay/Card.CardStruct` Card) 0.6)
    (`UserWidget.AddToViewport` _viewcardpreview 0)
    (else
      (`Widget.RemoveFromParent` _viewcardpreview)
      (`Widget.RemoveFromParent` _viewcardpreview))))

(fn `CreateDrageActorVisual`
  (params (`UseActorLocation?` :type Boolean))
  (returns (ReturnValue :type Boolean))
  (`/Engine/EditorBlueprintResources/StandardMacros.IsValid` (`self.TargetDragSelectionActor`)
    (:`Is Valid`
      _)
    (:`Is Not Valid`
      (`/Engine/EditorBlueprintResources/StandardMacros.IsValid` (`self.TakingControl`)
        (:`Is Valid`
          (bind _returnvalue (`|SpawnActorFromClass` "/Game/ACGCard/Blueprints/GamePlay/TargetDragSelection.TargetDragSelection_C" (`KismetMathLibrary.Conv_VectorToTransform` (select `bool` `UseActorLocation?` :`false` (`.Hit Result Location` (`/Game/ACGCard/Blueprints/Libs/Misc_FuncLib.MouseToWorldLocation` self)) :`true` (`self.K2_GetActorLocation` (`ActorComponent.GetOwner` (`self.TakingControl`))))) "Undefined" "OverrideRootScale" null null))
          (set `self.TargetDragSelectionActor` _returnvalue))
        (:`Is Not Valid`
          _))))
  (return (`KismetSystemLibrary.IsValid` (`self.TakingControl`))))

(fn `DetectCardInteraction`
  (bind _hitcontrol (`self.HitControl`))
  (bind _playerid (`/Game/ACGCard/Blueprints/Components/CardManager.PlayerId` (`self.CardManagerComponent`)))
  (bind _returnvalue (`self.SwitchValidCardControl` (`/Game/ACGCard/Blueprints/Libs/Misc_FuncLib.MouseToWorldLocation` self))
    (:`Is Valid`
      (bind _output_get (set `self.HitControl` _returnvalue))
      (`/Game/ACGCard/Blueprints/Libs/Card_MacroLib.CheckTurnPoint` _output_get
        (:`true`
          (`self.IsOwnPlayer` _output_get (`/Game/ACGCard/Blueprints/Components/CardManager.PlayerId` (`self.CardManagerComponent`))
            (:`true`
              (if (`self.bIsCardSelected`)
                (`/Engine/EditorBlueprintResources/StandardMacros.IsValid` (`self.TakingControl`)
                  (:`Is Valid`
                    (`/Game/ACGCard/Blueprints/Libs/Card_MacroLib.CheckCard` (`self.TakingControl`) (`self.HitControl`) :!via `Same?` :!label _label
                      (:`HasTurnpoint`
                        (bind _output_get_2 (set `self.RecevingControl` _hitcontrol))
                        (`self.SetCardSelection` _output_get_2 true _playerid))
                      (:`haven't Turnpoint`
                        (`self.SetCardInteraction` "NewEnumerator0" :!label _label_2))
                      (:`Is Same`
                        (goto _label_2))
                      (:`Is Not Same`
                        (`/Game/ACGCard/Blueprints/Libs/Card_MacroLib.Then`)
                        (goto _label)))
                    (return))
                  (:`Is Not Valid`
                    _))
                (else
                  (set `self.bIsCardSelected` true)
                  (`self.SetCardInteraction` "NewEnumerator1")))
              (bind _output_get_3 (set `self.TakingControl` _hitcontrol))
              (`self.SetCardSelection` _output_get_3 true _playerid))
            (:`false`
              (`/Engine/EditorBlueprintResources/StandardMacros.IsValid` (`self.TakingControl`)
                (:`Is Valid`
                  (goto _label :!via `Same?`))
                (:`Is Not Valid`
                  (goto _label_2))))))
        (:`false`
          (goto _label_2)))
      (return))))

(fn `DetectCardInteractionOnMove`
  (bind (_hit_result_hit_actor _hit_result_location) (`/Game/ACGCard/Blueprints/Libs/Misc_FuncLib.MouseToWorldLocation` self))
  (`self.EnableDragSelection`
    (:`IsDragging`
      _)
    (:`SetDragging`
      _))
  (bind _returnvalue (`self.SwitchValidCardControl` _hit_result_hit_actor)
    (:`Is Valid`
      (bind _output_get (set `self.HitControl` _returnvalue))
      (`/Game/ACGCard/Blueprints/Libs/Card_MacroLib.CheckCard` (`self.TakingControl`) _output_get :!label _label
        (:`HasTurnpoint`
          (`/Game/ACGCard/Blueprints/Libs/Card_MacroLib.Then`)
          (goto _label :!via `CheckAttack`))
        (:`haven't Turnpoint`
          _)
        (:`Can Attack`
          (`/Game/ACGCard/Blueprints/Libs/Card_MacroLib.Then`)
          (goto _label :!via `Same?`))
        (:`Can't Attack`
          (`self.CleanCardInteraction`))
        (:`Is Same`
          (bind _returnvalue_2 (`self.CreateDrageActorVisual` true :!label _label_2))
          (if _returnvalue_2
            (`/Game/ACGCard/Blueprints/GamePlay/TargetDragSelection.Set Selection Properties` (`self.TargetDragSelectionActor`) _hit_result_location (`KismetSystemLibrary.IsValid` (`self.RecevingControl`)))))
        (:`Is Not Same`
          (`self.SetCardSelection` (`self.RecevingControl`))
          (set `self.RecevingControl` (`self.HitControl`))
          (`self.SetCardSelection` (`self.RecevingControl`) true (`/Game/ACGCard/Blueprints/Components/CardManager.PlayerId` (`self.CardManagerComponent`)))
          (goto _label_2))))
    (:`Is Not Valid`
      (`self.SetCardSelection` (`self.RecevingControl`))
      (set `self.RecevingControl` null)
      (goto _label_2)))
  (return))

(fn `InitVariable`
  (`|ExecutionSequence`
    (:`then_0`
      (`|ExecutionSequence`
        (:`then_0`
          (bind _ascard_game_instance (cast `/Game/ACGCard/Blueprints/CardGameInstance` (`GameplayStatics.GetGameInstance`)))
          (set `self.Platform` (`/Game/ACGCard/Blueprints/CardGameInstance.Platform` _ascard_game_instance)))
        (:`then_1`
          (bind _ascard_game_state (cast `/Game/ACGCard/Blueprints/CardGameState` (`GameplayStatics.GetGameState`)))
          (set `self.CardGameStateRef` _ascard_game_state))))
    (:`then_1`
      (`/Engine/EditorBlueprintResources/StandardMacros.Can Execute Cosmetic Events`
        (:`True`
          (bind _returnvalue (`|CreateWidget` "/Game/ACGCard/Blueprints/Widgets/GamePlay/W_CardPreview.W_CardPreview_C" (`GameplayStatics.GetPlayerController` 0)))
          (set `self.ViewCardPreview` _returnvalue))))))

(fn `SetCardLocation`
  (params (HoldLocation :type "Vector Structure") (Card :type "/Game/ACGCard/Blueprints/GamePlay/Card Object Reference") (Rotation :type "Rotator Structure"))
  (bind _returnvalue (`GameplayStatics.GetWorldDeltaSeconds`))
  (bind _returnvalue_2 (`self.K2_GetActorLocation` Card))
  (bind _yaw (.yaw Rotation))
  (bind _returnvalue_3 (> _yaw 0.0))
  (bind _returnvalue_4 (/ (- (.x _returnvalue_2) (.x HoldLocation)) 5.0))
  (bind _returnvalue_5 (/ (- (.y _returnvalue_2) (.y HoldLocation)) 5.0))
  (`/Engine/EditorBlueprintResources/StandardMacros.IsValid` Card
    (:`Is Valid`
      (`self.K2_SetActorLocation` Card (`KismetMathLibrary.VInterpTo` _returnvalue_2 HoldLocation _returnvalue 10.0) false false) ; Set the Card in hand's location
      (if (`self.bEnableInHandMovementRotation`)
        (`self.K2_SetActorRotation` Card (`KismetMathLibrary.RInterpTo` (`self.K2_GetActorRotation` Card) (`KismetMathLibrary.MakeRotator` (select `bool` _returnvalue_3 :`false` _returnvalue_5 :`true` (* _returnvalue_5 -1.0)) (select `bool` _returnvalue_3 :`false` (* _returnvalue_4 -1.0) :`true` _returnvalue_4) _yaw) _returnvalue 5.0) false) ; Sets rotation of the card based on the movement speed of the mouse.
      ))
    (:`Is Not Valid`
      _))
  (return))

(fn `SetupGameUI`
  (if (`self.IsLocalPlayerController`)
    (bind _returnvalue (`|CreateWidget` "/Game/ACGCard/Blueprints/Widgets/GamePlay/W_PlayerGameUI.W_PlayerGameUI_C" self))
    (bind _output_get (set `self.PlayerGameUI` _returnvalue))
    (`UserWidget.AddToViewport` _output_get 2))
  (return))

(fn `UserConstructionScript`)

(fn `ValidateCardPlacementOnMove`
  (params (`Hit Actor` :type "Actor Object Reference"))
  (returns (Output_Get :type Boolean))
  (bind _targetcardplacement (`self.TargetCardPlacement`))
  (bind _targetcardplacement_2 (`self.TargetCardPlacement`))
  (bind _cardplacement (`self.CardPlacement`))
  (bind _output_get (set `self.HitActor` `Hit Actor`))
  (bind _ascard_placement (cast `/Game/ACGCard/Blueprints/GamePlay/CardPlacement` _output_get)
    (:`then`
      (bind _output_get_2 (set `self.CardPlacement` _ascard_placement))
      (if (== (`self.TargetCardPlacement`) (`self.CardPlacement`)) :!label _label
        (bind _return_index (`/Game/ACGCard/Blueprints/GamePlay/CardPlacement.CaculateShadowCardIndex` _targetcardplacement_2 (`self.PlayCard_Client_Ref`) :!label _label_2))
        (`/Game/ACGCard/Blueprints/GamePlay/CardPlacement.SetShadowCard` _targetcardplacement_2 _return_index)
        (set `self.TempInsertIndex` _return_index)
        (else
          (`self.ValidatePlacementOwner` (`/Game/ACGCard/Blueprints/Components/CardManager.PlayerId` (`self.CardManagerComponent`)) (`/Game/ACGCard/Blueprints/GamePlay/CardPlacement.PlayerId` _output_get_2) (`self.TempCardStruct`)
            (:`Both`
              (`/Engine/EditorBlueprintResources/StandardMacros.IsValid` _targetcardplacement :!label _label_3
                (:`Is Valid`
                  (if (not (== _targetcardplacement _cardplacement))
                    (set `self.TargetCardPlacement` _cardplacement :!label _label_4)))
                (:`Is Not Valid`
                  (goto _label_4)))
              (bind _output_get_3 (set `self.bIsValidClientDrop` true))
              (goto _label_2))
            (:`Self`
              (goto _label_3))
            (:`Oppenent`
              (goto _label_3))
            (:`None`
              (`self.CleanCardPlacement` :!label _label_5)
              (set `self.CardPlacement` null)
              (set `self.TargetCardPlacement` null)
              (set `self.bIsValidClientDrop` false))))))
    (:`CastFailed`
      (bind _ascard (cast `/Game/ACGCard/Blueprints/GamePlay/Card` _output_get)
        (:`then`
          (set `self.CardPlacement` (`/Game/ACGCard/Blueprints/GamePlay/Card.PlacementOwner` _ascard))
          (goto _label))
        (:`CastFailed`
          (goto _label_5)))))
  (return _output_get_3))

(fn `ValidateInteractionState`
  (returns (bValidInteraction :type Boolean))
  (set `self.bValidInteraction` false) ; Makes sure that the interaction is reliant on the checks after this point so be counted as valid.
  (if (`self.bIsCardSelected`)
    (`self.ValidateInteraction`
      (:`true`
        (set `self.bValidInteraction` true))
      (:`false`
        _)))
  (return (`self.bValidInteraction`)))